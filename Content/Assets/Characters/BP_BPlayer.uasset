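; Player character with clamped camera pitch and zoom, a two-press jump whose second press launches upward, and debug keys.
; Combat mode toggles only with a held item, messaging the AnimInstance and switching orient-to-movement.
; Tick drives a custom dispatcher whose bound handler turns the body toward control yaw once the aim offset exceeds a threshold, until nearly aligned.
; Weapon-mesh projectile spawning exists but is unwired.
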(event Custom|Custom%20Tick%201
  (params (DeltaSec :type Float%20%28single-precision%29))
  (bind _returnvalue (Pawn|GetControlRotation :!class /Script/Engine.Pawn))
  (bind _returnvalue_2 (Transformation|GetActorRotation))
  (bind _yaw (Math|Rotator|BreakRotator _returnvalue_2))
  (bind _yaw_2 (Math|Rotator|BreakRotator _returnvalue))
  (bind _returnvalue_3 (Math|Rotator|MakeRotator 0.0 0.0 _yaw))
  (bind _returnvalue_4 (Math|Rotator|MakeRotator 0.0 0.0 _yaw_2))
  (bind _returnvalue_5 (Math|Rotator|Delta(Rotator) _returnvalue_4 _returnvalue_3))
  (bind _yaw_3 (Math|Rotator|BreakRotator _returnvalue_5))
  ;[1 1 1] Auto-Rotation in Combat Mode
  (if (Variables|State|GetCombatMode?)
    (if (or (Variables|State|GetInAimOffsetRotation?) (> (Math|Float|Absolute(Float) _yaw_3) 7e+01))
      (Variables|State|SetInAimOffsetRotation? true)
      (Class|Actor|AddActorWorldRotation (Math|Interpolation|RInterpTo "0, 0, 0" _returnvalue_5 DeltaSec 5.0))
      (Variables|State|SetInAimOffsetRotation? (not (Math|Float|NearlyEqual(Float) _yaw_3 0.0 2.0))))))

(event EventBeginPlay
  ;[0.3824 1 0] BeginPlay + Tick
  (EventDispatchers|BindEventtoCustomTick (delegate Custom|Custom%20Tick%201)))

(event EventOnLanded
  (params (Hit :type Hit%20Result%20Structure%20%28by%20ref%29))
  ;[1 1 1] Jump Mechanics
  (Character|StopJumping)
  (Utilities|FlowControl|DoN 2) ; enters at Reset
)

(event EventTick
  (params (DeltaSeconds :type Float%20%28single-precision%29))
  ;[0.3824 1 0] BeginPlay + Tick
  (Default|CallCustomTick DeltaSeconds))

(event Input|ActionEvents|InputActionZoomIn
  (params (Key :type Key%20Structure :default "AnyKey"))
  (bind _cameraboom (Variables|Default|GetCameraBoom))
  ;[1 1 1] Camera Boom Control
  (:Pressed
    (Variables|/Script/Engine.SpringArmComponent|SetTargetArmLength _cameraboom (Math|Float|Clamp(Float) (- (Variables|/Script/Engine.SpringArmComponent|GetTargetArmLength _cameraboom) 5e+01) 1e+02 4e+02))))

(event Input|ActionEvents|InputActionZoomOut
  (params (Key :type Key%20Structure :default "AnyKey"))
  (bind _cameraboom (Variables|Default|GetCameraBoom))
  ;[1 1 1] Camera Boom Control
  (:Pressed
    (Variables|/Script/Engine.SpringArmComponent|SetTargetArmLength _cameraboom (Math|Float|Clamp(Float) (+ (Variables|/Script/Engine.SpringArmComponent|GetTargetArmLength _cameraboom) 5e+01) 1e+02 4e+02))))

(event Input|ActionEvents|InputActionJump
  (params (Key :type Key%20Structure :default "AnyKey"))
  ;[1 1 1] Jump Mechanics
  (:Pressed
    (Variables|State|SetJumpPressed? true)
    (bind _counter (Utilities|FlowControl|DoN 2)
      (:Exit
        (switch int _counter
          (:1
            (Development|PrintString 0 "Jump"))
          (:2
            (Character|LaunchCharacter "0, 0,700.000000" false false))))))
  (:Released
    (Variables|State|SetJumpPressed? false)))

(event Input|ActionEvents|InputActionAiming
  (params (Key :type Key%20Structure :default "AnyKey")))

(event Input|ActionEvents|InputActionToggleMode
  (params (Key :type Key%20Structure :default "AnyKey"))
  (bind _mesh (Variables|Character|GetMesh))
  (bind _charactermovement (Variables|Character|GetCharacterMovement))
  (bind _returnvalue (Components|SkeletalMesh|GetAnimInstance _mesh))
  ;[1 1 1] Combat Mode Toggle
  (:Pressed
    (if (Variables|Default|GetIsItemHeld)
      (if (Variables|State|GetCombatMode?)
        (Variables|State|SetCombatMode? false)
        (Class|CombatModeInterface|DisableCombatMode(Message) _returnvalue)
        (Variables|/Script/Engine.CharacterMovementComponent|SetbOrientRotationToMovement _charactermovement true)
        (Class|CombatModeInterface|UnEquipWeapon(Message) _returnvalue)
        (else
          (Class|CombatModeInterface|EquipWeapon(Message) _returnvalue)
          (Utilities|FlowControl|Delay 0 1.0)
          (Variables|State|SetCombatMode? true)
          (Class|CombatModeInterface|EnableCombatMode(Message) _returnvalue)
          (Variables|/Script/Engine.CharacterMovementComponent|SetbOrientRotationToMovement _charactermovement false)))
      (else
        (Development|PrintString 0 "NO ITEM, DUMMY!")))))

(event Input|AxisEvents|InputAxisLookUp
  (params (AxisValue :type Float%20%28single-precision%29))
  (bind _returnvalue (Pawn|GetControlRotation :!class /Script/Engine.Pawn))
  (bind (_roll _pitch _yaw) (Math|Rotator|BreakRotator _returnvalue))
  ;[1 1 1] Camera Boom Control
  (Pawn|SetControlRotation (Pawn|GetController) (Math|Rotator|MakeRotator _roll (Math|Float|ClampAngle (+ (* AxisValue -1.0) _pitch) -4e+01 4e+01) _yaw)))

(event Input|KeyboardEvents|V
  (params (Key :type Key%20Structure :default "AnyKey"))
  (bind _capsulecomponent (Variables|Default|GetCapsuleComponent))
  (:Pressed
    (Collision|LineTraceForObjects 0 "0, 0, 0" (+ (* (Math|Vector|GetForwardVector (Transformation|GetWorldRotation _capsulecomponent)) 1e+03) (Transformation|GetWorldLocation _capsulecomponent)) (Utilities|Array|MakeArray "ObjectTypeQuery3") false 0 "ForDuration")))

(event Input|KeyboardEvents|C
  (params (Key :type Key%20Structure :default "AnyKey"))
  ;[1 1 1] Debug Printing
  (:Pressed
    (Development|PrintString 0 (Utilities|String|ToString(Rotator) (Pawn|GetControlRotation :!class /Script/Engine.Pawn)))))

(fn ConstructionScript)

(fn JumpOutOfCombatMode
  (Variables|State|SetCombatMode? false)
  (Class|CombatModeInterface|DisableCombatMode(Message) (Components|SkeletalMesh|GetAnimInstance (Variables|Character|GetMesh)))
  (Variables|/Script/Engine.CharacterMovementComponent|SetbOrientRotationToMovement (Variables|Character|GetCharacterMovement) true)
  (Variables|Default|SetIsItemHeld false))