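; Grunt AI character that wanders the navmesh and carries a health bar turned toward the player.
; When movement is enabled, BeginPlay loops AIMoveTo to random nearby points, pausing between moves.
; Tick updates the bar's fill and yaws its scene component toward the player.
; CalculateDamage always uses base damage, then ApplyTotalDamage lowers health and flags the anim blueprint's hit reaction; CheckForDeath, uncalled here, only clamps health at zero.
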(event Custom|Calculate%20Damage
  ;[1 0.1006 0.2251] Damage
  (switch int 0
    (:0
      (Variables|Default|SetTotalDamage (Variables|Default|GetDamageBase)))
    (:1
      _)
    (:2
      _))
  (CallFunction|ApplyTotalDamage))

(event Custom|ApplyTotalDamage
  ;[1 0.1006 0.2251] Damage
  (if (>= (- (Variables|Default|GetCurrentHealth) (Variables|Default|GetTotalDamage)) (Variables|Default|GetMaxtHealth))
    (Variables|Default|SetCurrentHealth 0)
    (else
      (Variables|Default|SetCurrentHealth (- (Variables|Default|GetCurrentHealth) (Variables|Default|GetTotalDamage)))
      (bind _asue4asp_hero_tpp_anim_blueprint (Utilities|Casting|CastToUE4ASP_HeroTPP_AnimBlueprint (Components|SkeletalMesh|GetAnimInstance (Variables|Character|GetMesh))))
      (Variables|/Game/AnimStarterPack/UE4ASP_HeroTPP_AnimBlueprint.UE4ASP_HeroTPP_AnimBlueprint_C|SetHitByAttack? _asue4asp_hero_tpp_anim_blueprint true))))

(event EventTick
  (params (DeltaSeconds :type Float%20%28single-precision%29))
  (bind _scene (Variables|Default|GetScene))
  ;[0.155 0.4406 1] - Set % + Rotate Towards Player
  (bind _asaihealth_bar (Utilities|Casting|CastToAIHealthBar (UserInterface|GetUserWidgetObject (Variables|Default|GetHealthBar))))
  (Progress|SetPercent (Variables|/Game/Blueprints/AIHealthBar.AIHealthBar_C|GetProgressBar_169 _asaihealth_bar) (/ (Math|Conversions|ToFloat(Byte) (Variables|Default|GetCurrentHealth)) (Math|Conversions|ToFloat(Byte) (Variables|Default|GetMaxtHealth))))
  (Transformation|SetWorldRotation _scene (Math|Rotator|MakeRotator 0.0 0.0 (.Yaw (Math|Rotator|BreakRotator (Math|Rotator|FindLookatRotation (Transformation|GetWorldLocation _scene) (Transformation|GetActorLocation (Game|GetPlayerCharacter 0)))))) false false))

(event EventBeginPlay
  ;[1 1 1] Find Random Point in Radius to Move to
  (if (Variables|Default|GetMovementOn?)
    (AI|AIMoveTo self (Class|NavigationSystem|GetRandomPointinNavigableRadius (Transformation|GetActorLocation) 1e+03) 0 5.0 false :!label _label
      (:OnSuccess
        _)
      (:OnFail
        _))
    (Utilities|FlowControl|Delay 1.0)
    (goto _label)))

(fn ConstructionScript
  (bind _output_get (Variables|Default|SetMaxtHealth 100))
  (Variables|Default|SetCurrentHealth _output_get))

(fn CheckforDeath
  (if (<= (Variables|Default|GetCurrentHealth) 0)
    (Variables|Default|SetCurrentHealth 0)))