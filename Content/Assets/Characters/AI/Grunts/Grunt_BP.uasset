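; Grunt AI character that attacks with cast projectiles and can be squished by the player.
; Attack, damage and death events play montages, with damage and death then passing to the parent class.
; Fire spawns a projectile at the Caster component, aimed by the supplied rotation, and copies the Caster's particle template to its emitter.
; Capsule overlap with a size 5 player enables mesh physics and triggers death.
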(event OnComponentBeginOverlap(CapsuleComponent)
  (params (OtherActor :type Actor%20Object%20Reference) (OtherComp :type Primitive%20Component%20Object%20Reference) (OtherBodyIndex :type Integer) (bFromSweep :type Boolean) (SweepResult :type Hit%20Result%20Structure%20%28by%20ref%29))
  ;[1 1 1] Squish when Overlapped by Player with Size of 5
  (bind _asbp_bplayer (Utilities|Casting|CastToBP_BPlayer OtherActor))
  (if (== (Variables|/Game/Assets/Characters/BP_BPlayer.BP_BPlayer_C|GetSize _asbp_bplayer) 5)
    (Physics|SetSimulatePhysics (Variables|Character|GetMesh) true)
    (CallFunction|DIDeath)))

(event EventDIAttack
  ;[1 1 1] Play attack Montage when Attack Triggered
  (Animation|PlayAnimMontage "/Game/Assets/Characters/AI/InfinityBladeAdversaries/Enemy/Enemy_Gruntling/Enemy_Gruntling_Animation/CastMontage.CastMontage" 1.0 "None"))

(event EventDIFire
  (params (LookAtRotation :type Rotator))
  (bind _caster (Variables|Default|GetCaster))
  (bind _returnvalue (Transformation|GetWorldTransform _caster))
  (bind (_location _rotation _scale) (Math|Transform|BreakTransform _returnvalue))
  ;[1 1 1] Spawn Cast Porjectile when Fire is Called
  (bind _returnvalue_2 (Game|SpawnActorfromClass "/Game/Assets/Items/BluePrints/WeaponBPs/Projectiles/BulletsAndCasts/CastProjectile.CastProjectile_C" (Math|Transform|MakeTransform _location LookAtRotation _scale) "Undefined" 0 0))
  (Effects|Components|ParticleSystem|SetTemplate (Variables|/Game/Assets/Items/BluePrints/WeaponBPs/Projectiles/BulletsAndCasts/CastProjectile.CastProjectile_C|GetEmitter _returnvalue_2) (Variables|/Script/Engine.ParticleSystemComponent|GetTemplate _caster))
  (Variables|Default|SetProjectile _returnvalue_2))

(event EventDIDamage
  (params (Sender :type Actor%20Object%20Reference) (Impulse? :type Boolean) (IV :type Vector) (HB :type Name) (HL :type Vector))
  (Animation|PlayAnimMontage "/Game/Assets/Characters/AI/InfinityBladeAdversaries/Enemy/Enemy_Gruntling/Enemy_Gruntling_Animation/HitMontage.HitMontage" 1.0 "None")
  (|CallParentFunction Sender Impulse? IV HB HL))

(event EventDIDeath
  (Animation|PlayAnimMontage "/Game/Assets/Characters/AI/InfinityBladeAdversaries/Enemy/Enemy_Gruntling/Enemy_Gruntling_Animation/DeathMontage.DeathMontage" 1.0 "None")
  (|CallParentFunction))

(fn ConstructionScript
  (|CallParentFunction))