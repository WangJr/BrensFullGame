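; BP_DItem is an item actor that a BCharacter picks up and carries on its mesh.
; The OverlapDetect component's begin and end overlap events toggle input for player controller 0, with debug prints.
; Pressing Pickup Item while the character's hands are free relaxes collision and snaps the item to the WeaponHolster socket.
; It then passes itself, its item type and the held flag to the character.
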(event OnComponentBeginOverlap(OverlapDetect)
  (params (OtherActor :type Actor%20Object%20Reference) (OtherComp :type Primitive%20Component%20Object%20Reference) (OtherBodyIndex :type Integer) (bFromSweep :type Boolean) (SweepResult :type Hit%20Result%20Structure%20%28by%20ref%29))
  ;[1 1 1] Enable/Disable Input
  (Utilities|Casting|CastToBCharacterClass (Utilities|GetClass OtherActor)
    (:then
      (Development|PrintString "ENTERING!!!!!")
      (Input|EnableInput (Game|GetPlayerController 0)))
    (:CastFailed
      (Development|PrintString "Hello"))))

(event OnComponentEndOverlap(OverlapDetect)
  (params (OtherActor :type Actor%20Object%20Reference) (OtherComp :type Primitive%20Component%20Object%20Reference) (OtherBodyIndex :type Integer))
  ;[1 1 1] Enable/Disable Input
  (Utilities|Casting|CastToBCharacterClass (Utilities|GetClass OtherActor)
    (:then
      (Development|PrintString "Exiting!!!!!!!")
      (Input|DisableInput (Game|GetPlayerController 0) 0))
    (:CastFailed
      (Development|PrintString "Hello"))))

(event Input|ActionEvents|InputActionPickupItem
  (params (Key :type Key%20Structure :default "AnyKey"))
  ;[1 1 1] Pickup Item
  (:Pressed
    (bind _asbcharacter (Utilities|Casting|CastToBCharacter (stale OnComponentBeginOverlap(OverlapDetect) OtherActor)))
    (if (not (Variables|/Script/BrensFullGame.BCharacter|GetIsItemHeld _asbcharacter))
      (Collision|SetCollisionResponsetoAllChannels (Variables|Default|GetDItemMesh) "ECR_Overlap")
      (Collision|SetCollisionResponsetoAllChannels (Variables|Default|GetOverlapDetect) "ECR_Ignore")
      (Class|Actor|AttachRootComponentto (Variables|/Script/Engine.Character|GetMesh _asbcharacter) "WeaponHolster" "SnapToTarget" true)
      (Class|BCharacter|SetValues _asbcharacter self (Variables|Default|GetItemType) true))))

(fn ConstructionScript)