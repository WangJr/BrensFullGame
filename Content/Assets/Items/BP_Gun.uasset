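; BP_Gun is a gun item that a BCharacter picks up with the Pickup Item input.
; Overlapping OverlapDetect enables the gun's input for player 0, while leaving calls DisableInput on that player controller, with debug prints on both.
; Pickup uses the overlap's OtherActor, switches mesh and detector collision to Overlap, snaps the gun to the WeaponHolster socket and sets itself as HeldItem.
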(event OnComponentBeginOverlap(OverlapDetect)
  (params (OtherActor :type Actor%20Object%20Reference) (OtherComp :type Primitive%20Component%20Object%20Reference) (OtherBodyIndex :type Integer) (bFromSweep :type Boolean) (SweepResult :type Hit%20Result%20Structure%20%28by%20ref%29))
  (Utilities|Casting|CastToBCharacterClass (Utilities|GetClass OtherActor)
    (:then
      (Development|PrintString "ENTERING!!!!!")
      (Input|EnableInput (Game|GetPlayerController 0)))
    (:CastFailed
      (Development|PrintString "Hello"))))

(event OnComponentEndOverlap(OverlapDetect)
  (params (OtherActor :type Actor%20Object%20Reference) (OtherComp :type Primitive%20Component%20Object%20Reference) (OtherBodyIndex :type Integer))
  (Utilities|Casting|CastToBCharacterClass (Utilities|GetClass OtherActor)
    (:then
      (Development|PrintString "Exiting!!!!!!!")
      (Input|DisableInput (Game|GetPlayerController 0) 0))
    (:CastFailed
      (Development|PrintString "Hello"))))

(event Input|ActionEvents|InputActionPickupItem
  (params (Key :type Key%20Structure :default "AnyKey"))
  (:Pressed
    (bind _asbcharacter (Utilities|Casting|CastToBCharacter (stale OnComponentBeginOverlap(OverlapDetect) OtherActor)))
    (Collision|SetCollisionResponsetoAllChannels (Variables|SkeletalMeshActor|GetSkeletalMeshComponent) "ECR_Overlap")
    (Collision|SetCollisionResponsetoAllChannels (Variables|Default|GetOverlapDetect) "ECR_Overlap")
    (Class|Actor|AttachRootComponentto (Variables|/Script/Engine.Character|GetMesh _asbcharacter) "WeaponHolster" "SnapToTarget" true)
    (Variables|/Script/BrensFullGame.BCharacter|SetHeldItem _asbcharacter self)))

(fn ConstructionScript)