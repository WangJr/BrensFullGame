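; BP_SItem is a pickup item that the player character can attach to its body.
; Overlap begin and end events on OverlapDetect toggle input through player controller 0 after a BCharacter class check, printing debug messages.
; The Pickup Item action adjusts mesh and trigger collision, then snaps the item to the overlapping character's WeaponHolster socket.
; It then passes itself, its ItemType and a holding flag to the character.
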(event OnComponentEndOverlap(OverlapDetect)
  (params (OtherActor :type Actor%20Object%20Reference) (OtherComp :type Primitive%20Component%20Object%20Reference) (OtherBodyIndex :type Integer))
  (Utilities|Casting|CastToBCharacterClass (Utilities|GetClass OtherActor)
    (:then
      (Development|PrintString "Exiting!!!!!!!")
      (Input|DisableInput (Game|GetPlayerController 0) 0))
    (:CastFailed
      (Development|PrintString "Hello"))))

(event OnComponentBeginOverlap(OverlapDetect)
  (params (OtherActor :type Actor%20Object%20Reference) (OtherComp :type Primitive%20Component%20Object%20Reference) (OtherBodyIndex :type Integer) (bFromSweep :type Boolean) (SweepResult :type Hit%20Result%20Structure%20%28by%20ref%29))
  (Utilities|Casting|CastToBCharacterClass (Utilities|GetClass OtherActor)
    (:then
      (Development|PrintString "ENTERING!!!!!")
      (Input|EnableInput (Game|GetPlayerController 0)))
    (:CastFailed
      (Development|PrintString "Hello"))))

(event EventBeginPlay)

(event EventActorBeginOverlap
  (params (OtherActor :type Actor%20Object%20Reference)))

(event EventTick
  (params (DeltaSeconds :type Float%20%28single-precision%29)))

(event Input|ActionEvents|InputActionPickupItem
  (params (Key :type Key%20Structure :default "AnyKey"))
  (:Pressed
    (bind _asbcharacter (Utilities|Casting|CastToBCharacter (stale OnComponentBeginOverlap(OverlapDetect) OtherActor)))
    (Collision|SetCollisionResponsetoAllChannels (Variables|Default|GetSItemMesh) "ECR_Overlap")
    (Collision|SetCollisionResponsetoAllChannels (Variables|Default|GetOverlapDetect) "ECR_Ignore")
    (Class|Actor|AttachRootComponentto (Variables|/Script/Engine.Character|GetMesh _asbcharacter) "WeaponHolster" "SnapToTarget" true)
    (Class|BCharacter|SetValues _asbcharacter self (Variables|Default|GetItemType) true)))

(fn ConstructionScript)