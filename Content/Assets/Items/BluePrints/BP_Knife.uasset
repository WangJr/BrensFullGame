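; BP_Knife is a knife item whose blade overlap knocks characters other than player 0 into physics simulation.
; On overlap with such a BCharacter, it prints a hit message, enables physics on the character's mesh and applies an impulse scaled from the knife's velocity.
; TurnOnBlade toggles the blade's collision, so hits can be switched on and off.
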(event OnComponentBeginOverlap(BladeCollision)
  (params (OtherActor :type Actor%20Object%20Reference) (OtherComp :type Primitive%20Component%20Object%20Reference) (OtherBodyIndex :type Integer) (bFromSweep :type Boolean) (SweepResult :type Hit%20Result%20Structure%20%28by%20ref%29))
  (if (!= OtherActor (Game|GetPlayerCharacter 0))
    (Utilities|Casting|CastToBCharacter OtherActor)
    (Development|PrintString 0 "Thats a HIT!")
    (bind _asbcharacter (Utilities|Casting|CastToBCharacter OtherActor))
    (Physics|SetSimulatePhysics (Variables|/Script/Engine.Character|GetMesh _asbcharacter) true)
    (Physics|AddImpulseatLocation (Variables|/Script/Engine.Character|GetMesh _asbcharacter) (* (Transformation|GetVelocity) 1e+01) (Transformation|GetWorldLocation (Variables|/Script/Engine.Character|GetMesh _asbcharacter)) "None")))

(fn ConstructionScript
  (|CallParentFunction))

(fn TurnonBlade
  (params (On? :type Boolean))
  (bind _bladecollision (Variables|Default|GetBladeCollision))
  (if On?
    (Collision|SetCollisionEnabled _bladecollision "QueryAndPhysics")
    (else
      (Collision|SetCollisionEnabled _bladecollision "NoCollision"))))