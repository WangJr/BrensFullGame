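; Pickup item that the player can attach to the character's WeaponHolster socket, drop and attack with.
; Overlap events toggle the item's own input and store the current player.
; F alternates through a DoN counter between pickup, which registers the item on the character, and drop, which exits combat mode, with SetCollision switching overlap collision and mesh physics.
; Attack input sets the player's attacking flag and messages its AnimInstance.
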(event OnComponentEndOverlap(OverlapDetect)
  (params (OtherActor :type Actor%20Object%20Reference) (OtherComp :type Primitive%20Component%20Object%20Reference) (OtherBodyIndex :type Integer))
  ;[1 1 1] Enable/Disable Input
  (Utilities|Casting|CastToBCharacterClass (Utilities|GetClass OtherActor))
  (Development|PrintString "Exiting!!!!!!!")
  (Input|DisableInput (Game|GetPlayerController 0)))

(event OnComponentBeginOverlap(OverlapDetect)
  (params (OtherActor :type Actor%20Object%20Reference) (OtherComp :type Primitive%20Component%20Object%20Reference) (OtherBodyIndex :type Integer) (bFromSweep :type Boolean) (SweepResult :type Hit%20Result%20Structure%20%28by%20ref%29))
  ;[1 1 1] Enable/Disable Input
  (Utilities|Casting|CastToBCharacterClass (Utilities|GetClass OtherActor))
  (Variables|Default|SetCurrentPlayer OtherActor)
  (Development|PrintString "ENTERING!!!!!")
  (Input|EnableInput (Game|GetPlayerController 0)))

(event Input|ActionEvents|InputActionAttack
  (params (Key :type Key%20Structure :default "AnyKey"))
  (bind _currentplayer (Variables|Default|GetCurrentPlayer))
  ;[1 1 1] Item Attack
  (:Pressed
    (bind _asbp_bplayer (Utilities|Casting|CastToBP_BPlayer _currentplayer))
    (if (Variables|/Script/BrensFullGame.BCharacter|GetIsItemHeld _asbp_bplayer)
      (Class|CombatModeInterface|AttackStart(Message) (Components|SkeletalMesh|GetAnimInstance (Variables|/Script/Engine.Character|GetMesh _asbp_bplayer)))
      (Variables|/Game/Assets/Characters/BP_BPlayer.BP_BPlayer_C|SetAttacking? _asbp_bplayer true)
      (Development|PrintString "Attacking")))
  (:Released
    (bind _asbp_bplayer_2 (Utilities|Casting|CastToBP_BPlayer _currentplayer))
    (Variables|/Game/Assets/Characters/BP_BPlayer.BP_BPlayer_C|SetAttacking? _asbp_bplayer_2 false)
    (Class|CombatModeInterface|AttackEnd(Message) (Components|SkeletalMesh|GetAnimInstance (Variables|/Script/Engine.Character|GetMesh _asbp_bplayer)))
    (Development|PrintString "Stoppinglo")))

(event Input|KeyboardEvents|F
  (params (Key :type Key%20Structure :default "AnyKey"))
  (bind _currentplayer (Variables|Default|GetCurrentPlayer))
  ;[1 1 1] Pickup/Drop Item
  (:Pressed
    (bind _counter (Utilities|FlowControl|DoN 2 :!label _label)
      (:Exit
        (switch int _counter
          (:1
            (bind _asbcharacter (Utilities|Casting|CastToBCharacter _currentplayer)
              (:then
                (if (Variables|/Script/BrensFullGame.BCharacter|GetIsItemHeld _asbcharacter)
                  (Development|PrintString "E5")
                  (else
                    (CallFunction|SetCollision false)
                    (Class|Actor|AttachRootComponentto (Variables|/Script/Engine.Character|GetMesh _asbcharacter) "WeaponHolster" "SnapToTarget" true)
                    (Class|BCharacter|SetValues _asbcharacter self (Variables|Default|GetItemType) true)
                    (Input|EnableInput (Game|GetPlayerController 0)))))
              (:CastFailed
                (Development|PrintString "E4"))))
          (:2
            (bind _asbp_bplayer (Utilities|Casting|CastToBP_BPlayer _currentplayer))
            (Development|PrintString "Input is on Item")
            (Class|Actor|DetachRootComponentfromParent true)
            (Utilities|FlowControl|Delay 0.2)
            (CallFunction|SetCollision true)
            (Default|JumpOutOfCombatMode _asbp_bplayer)
            (goto _label Reset)))))))

(fn ConstructionScript)

(fn SetCollision
  (params (On? :type Boolean))
  (if On?
    (Variables|Default|SetEnableCollisionE "QueryAndPhysics")
    (else
      (Variables|Default|SetEnableCollisionE "NoCollision")))
  (Collision|SetCollisionEnabled (Variables|Default|GetOverlapDetect) (Variables|Default|GetEnableCollisionE))
  (Physics|SetSimulatePhysics (Variables|Default|GetSItemMesh) On?))