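; Time bubble actor whose sphere overlap changes time for characters and slows projectiles inside it.
; The Slow flag decides whether characters get reduced CustomTimeDilation inside or outside the sphere.
; Chameleon and SM projectiles always lose gravity and most velocity on entry, and blunt ones also spin slower.
; Exit restores them from one shared StoredVelocity, so the last entry overwrites earlier ones; SM physics simulation stays off.
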(event OnComponentBeginOverlap(Sphere)
  (params (OtherActor :type Actor%20Object%20Reference) (OtherComp :type Primitive%20Component%20Object%20Reference) (OtherBodyIndex :type Integer) (bFromSweep :type Boolean) (SweepResult :type Hit%20Result%20Structure%20%28by%20ref%29))
  (if (Variables|Default|GetSlow?)
    (Variables|Default|SetCTD 0.2)
    (else
      (Variables|Default|SetCTD 1.0)))
  (bind _asbcharacter (Utilities|Casting|CastToBCharacter OtherActor)
    (:then
      (Variables|/Script/Engine.Actor|SetCustomTimeDilation _asbcharacter (Variables|Default|GetCTD)))
    (:CastFailed
      (bind _asbp_chameleon_projectile_base (Utilities|Casting|CastToBP_ChameleonProjectileBASE OtherActor)
        (:then
          (Variables|Default|SetStoredVelocity (Variables|/Script/Engine.MovementComponent|GetVelocity (Variables|/Game/Assets/Items/BluePrints/WeaponBPs/Projectiles/BP_ChameleonProjectileBASE.BP_ChameleonProjectileBASE_C|GetProjectileMovement _asbp_chameleon_projectile_base)))
          (Variables|/Script/Engine.ProjectileMovementComponent|SetProjectileGravityScale (Variables|/Game/Assets/Items/BluePrints/WeaponBPs/Projectiles/BP_ChameleonProjectileBASE.BP_ChameleonProjectileBASE_C|GetProjectileMovement _asbp_chameleon_projectile_base) 0.0)
          (Variables|/Script/Engine.MovementComponent|SetVelocity (Variables|/Game/Assets/Items/BluePrints/WeaponBPs/Projectiles/BP_ChameleonProjectileBASE.BP_ChameleonProjectileBASE_C|GetProjectileMovement _asbp_chameleon_projectile_base) (* (Variables|/Script/Engine.MovementComponent|GetVelocity (Variables|/Game/Assets/Items/BluePrints/WeaponBPs/Projectiles/BP_ChameleonProjectileBASE.BP_ChameleonProjectileBASE_C|GetProjectileMovement _asbp_chameleon_projectile_base)) 0.1))
          (bind _asbp_dws_blunt_projectile (Utilities|Casting|CastToBP_DWS_BluntProjectile _asbp_chameleon_projectile_base))
          (Variables|/Game/Assets/Items/BluePrints/WeaponBPs/Projectiles/DS/BP_DWS_BluntProjectile.BP_DWS_BluntProjectile_C|SetDegPerSec _asbp_dws_blunt_projectile (/ (Variables|/Game/Assets/Items/BluePrints/WeaponBPs/Projectiles/DS/BP_DWS_BluntProjectile.BP_DWS_BluntProjectile_C|GetDegPerSec _asbp_dws_blunt_projectile) 5.0)))
        (:CastFailed
          (bind _asbp_smprojectile_base (Utilities|Casting|CastToBP_SMProjectileBASE OtherActor))
          (Physics|SetSimulatePhysics (Variables|/Game/Assets/Items/BluePrints/WeaponBPs/Projectiles/BP_SMProjectileBASE.BP_SMProjectileBASE_C|GetSphere _asbp_smprojectile_base) false)
          (Variables|Default|SetStoredVelocity (Variables|/Script/Engine.MovementComponent|GetVelocity (Variables|/Game/Assets/Items/BluePrints/WeaponBPs/Projectiles/BP_SMProjectileBASE.BP_SMProjectileBASE_C|GetProjectileMovement _asbp_smprojectile_base)))
          (Variables|/Script/Engine.ProjectileMovementComponent|SetProjectileGravityScale (Variables|/Game/Assets/Items/BluePrints/WeaponBPs/Projectiles/BP_SMProjectileBASE.BP_SMProjectileBASE_C|GetProjectileMovement _asbp_smprojectile_base) 0.0)
          (Variables|/Script/Engine.MovementComponent|SetVelocity (Variables|/Game/Assets/Items/BluePrints/WeaponBPs/Projectiles/BP_SMProjectileBASE.BP_SMProjectileBASE_C|GetProjectileMovement _asbp_smprojectile_base) (* (Variables|/Script/Engine.MovementComponent|GetVelocity (Variables|/Game/Assets/Items/BluePrints/WeaponBPs/Projectiles/BP_SMProjectileBASE.BP_SMProjectileBASE_C|GetProjectileMovement _asbp_smprojectile_base)) 0.1)))))))

(event OnComponentEndOverlap(Sphere)
  (params (OtherActor :type Actor%20Object%20Reference) (OtherComp :type Primitive%20Component%20Object%20Reference) (OtherBodyIndex :type Integer))
  (if (Variables|Default|GetSlow?)
    (Variables|Default|SetCTD 1.0)
    (else
      (Variables|Default|SetCTD 0.2)))
  (bind _asbcharacter (Utilities|Casting|CastToBCharacter OtherActor)
    (:then
      (Variables|/Script/Engine.Actor|SetCustomTimeDilation _asbcharacter (Variables|Default|GetCTD)))
    (:CastFailed
      (bind _asbp_chameleon_projectile_base (Utilities|Casting|CastToBP_ChameleonProjectileBASE OtherActor)
        (:then
          (Variables|/Script/Engine.MovementComponent|SetVelocity (Variables|/Game/Assets/Items/BluePrints/WeaponBPs/Projectiles/BP_ChameleonProjectileBASE.BP_ChameleonProjectileBASE_C|GetProjectileMovement _asbp_chameleon_projectile_base) (Variables|Default|GetStoredVelocity))
          (Variables|/Script/Engine.ProjectileMovementComponent|SetProjectileGravityScale (Variables|/Game/Assets/Items/BluePrints/WeaponBPs/Projectiles/BP_ChameleonProjectileBASE.BP_ChameleonProjectileBASE_C|GetProjectileMovement _asbp_chameleon_projectile_base) 1.0)
          (bind _asbp_dws_blunt_projectile (Utilities|Casting|CastToBP_DWS_BluntProjectile _asbp_chameleon_projectile_base))
          (Variables|/Game/Assets/Items/BluePrints/WeaponBPs/Projectiles/DS/BP_DWS_BluntProjectile.BP_DWS_BluntProjectile_C|SetDegPerSec _asbp_dws_blunt_projectile (* (Variables|/Game/Assets/Items/BluePrints/WeaponBPs/Projectiles/DS/BP_DWS_BluntProjectile.BP_DWS_BluntProjectile_C|GetDegPerSec _asbp_dws_blunt_projectile) 5.0)))
        (:CastFailed
          (bind _asbp_smprojectile_base (Utilities|Casting|CastToBP_SMProjectileBASE OtherActor))
          (Variables|/Script/Engine.MovementComponent|SetVelocity (Variables|/Game/Assets/Items/BluePrints/WeaponBPs/Projectiles/BP_SMProjectileBASE.BP_SMProjectileBASE_C|GetProjectileMovement _asbp_smprojectile_base) (Variables|Default|GetStoredVelocity))
          (Variables|/Script/Engine.ProjectileMovementComponent|SetProjectileGravityScale (Variables|/Game/Assets/Items/BluePrints/WeaponBPs/Projectiles/BP_SMProjectileBASE.BP_SMProjectileBASE_C|GetProjectileMovement _asbp_smprojectile_base) 1.0))))))

(event EventBeginPlay)

(event EventActorBeginOverlap
  (params (OtherActor :type Actor%20Object%20Reference)))

(event EventTick
  (params (DeltaSeconds :type Float%20%28single-precision%29)))

(fn ConstructionScript)