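; Axe weapon Blueprint that deals melee damage to BCharacters and assigns an axe projectile class.
; While attacking, Tick line-traces between previous and current blade points interpolated from sockets, seeding them once per trace reset.
; Blade hits deal TotalDamage, with a swing-direction impulse if health exceeds BaseDamage; otherwise, fallback traces on other hit locations deal light handle damage.
; The first character hit ends the attack, and a bound event re-enables mesh collision.
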(event Custom|ToggleSKMeshCollision
  (Collision|SetCollisionEnabled (Variables|Default|GetSkeletalMesh) "QueryAndPhysics"))

(event EventBeginPlay
  (EventDispatchers|BindEventtoToggleCollisionMesh (delegate Custom|ToggleSKMeshCollision)))

(event EventActorBeginOverlap
  (params (OtherActor :type Actor%20Object%20Reference)))

(event EventTick
  (params (DeltaSeconds :type Float%20%28single-precision%29))
  (if (Variables|Default|GetAttack?)
    (Utilities|FlowControl|Sequence
      (:then_0
        (Utilities|FlowControl|DoOnce false
          (:Completed
            (CallFunction|CalculateHitLocations)
            (CallFunction|CalculateSharp)
            (Variables|Default|SetOldSharps (Variables|Default|GetNewSharps))
            (Variables|Default|SetOldHitLocations (Variables|Default|GetNewHitLocations)))))
      (:then_1
        (CallFunction|CalculateHitLocations)
        (CallFunction|CalculateSharp)
        (CallFunction|RunSharps)
        (Variables|Default|SetOldSharps (Variables|Default|GetNewSharps))
        (Variables|Default|SetOldHitLocations (Variables|Default|GetNewHitLocations))))))

(event EventTraceReset
  (Utilities|FlowControl|DoOnce false) ; enters at Reset
)

(fn ConstructionScript
  (|CallParentFunction)
  (Variables|Default|SetProjectileClass "/Game/Assets/Items/BluePrints/WeaponBPs/Projectiles/DS/Axe/BP_DWS_AxeProjectile.BP_DWS_AxeProjectile_C")
  (Variables|Default|SetBaseDamage 3e+01))

(fn CalculateSharp
  (bind _skeletalmesh (Variables|Default|GetSkeletalMesh))
  (bind _returnvalue (Transformation|GetSocketLocation _skeletalmesh "SBase"))
  (bind _returnvalue_2 (Transformation|GetSocketLocation _skeletalmesh "STip"))
  (bind _returnvalue_3 (- _returnvalue_2 _returnvalue))
  (Variables|Default|SetNewSharps (Utilities|Array|MakeArray _returnvalue_2 (+ (* _returnvalue_3 0.75) _returnvalue) (+ (* _returnvalue_3 0.5) _returnvalue) (+ (* _returnvalue_3 0.25) _returnvalue) _returnvalue)))

(fn RunSharps
  (bind _index (Utilities|FlowControl|ForLoopwithBreak 0 4 :!label _label)
    (:LoopBody
      (bind (_outhit _returnvalue) (Collision|LineTraceForObjects (Utilities|Array|Get(acopy) (Variables|Default|GetOldSharps) _index) (Utilities|Array|Get(acopy) (Variables|Default|GetNewSharps) _index) (Utilities|Array|MakeArray "ObjectTypeQuery3") false (Utilities|Array|MakeArray (Variables|Default|GetCurrentPlayer)) "None"))
      (if _returnvalue
        (Variables|Default|SetPHit? true)
        (bind _asbcharacter (Utilities|Casting|CastToBCharacter (.HitActor (Collision|BreakHitResult _outhit))))
        (if (> (Variables|/Script/BrensFullGame.BCharacter|GetCurrentHealth _asbcharacter) (Variables|Default|GetBaseDamage))
          (Variables|Default|SetImp true)
          (Variables|Default|SetImpVec (* (Math|Vector|Normalize (- (Utilities|Array|Get(acopy) (Variables|Default|GetNewSharps) _index) (Utilities|Array|Get(acopy) (Variables|Default|GetOldSharps) _index))) 1e+03))
          (else
            (Variables|Default|SetImp false)
            (Variables|Default|SetImpVec "0, 0, 0")))
        (Class|BCharacter|SetPlayerDamage _asbcharacter (Variables|Default|GetTotalDamage) 1 0.0 self)
        (Variables|Default|SetAttack? false)
        (Class|DamageInterface|DIDamage(Message) _asbcharacter (Variables|Default|GetCurrentPlayer) (Variables|Default|GetImp) (Variables|Default|GetImpVec) (.HitBoneName (Collision|BreakHitResult _outhit)) "0, 0, 0")
        (goto _label Break)))
    (:Completed
      (if (Variables|Default|GetPHit?)
        (Variables|Default|SetPHit? false)
        (else
          (bind _index_2 (Utilities|FlowControl|ForLoopwithBreak 0 4 :!label _label_2)
            (:LoopBody
              (bind (_outhit_2 _returnvalue_2) (Collision|LineTraceForObjects (Utilities|Array|Get(acopy) (Variables|Default|GetOldHitLocations) _index_2) (Utilities|Array|Get(acopy) (Variables|Default|GetNewHitLocations) _index_2) (Utilities|Array|MakeArray "ObjectTypeQuery3") false (Utilities|Array|MakeArray (Variables|Default|GetCurrentPlayer)) "None"))
              (if _returnvalue_2
                (bind _asbcharacter_2 (Utilities|Casting|CastToBCharacter (.HitActor (Collision|BreakHitResult _outhit_2))))
                (Development|PrintString "HitHandle")
                (Class|BCharacter|SetPlayerDamage _asbcharacter_2 5.0 0 0.0 self)
                (Variables|Default|SetAttack? false)
                (Class|DamageInterface|DIDamage(Message) _asbcharacter_2 (Variables|Default|GetCurrentPlayer) false "0, 0, 0" (.HitBoneName (Collision|BreakHitResult _outhit_2)) "0, 0, 0")
                (goto _label_2 Break)))))))))