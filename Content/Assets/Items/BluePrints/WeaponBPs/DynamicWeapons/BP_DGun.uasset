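; BP_DGun is a gun Blueprint among the dynamic weapons that tracks clip and reserve ammo.
; Its construction script runs the parent's, then fills the clip to ClipSize.
; UpdateAmmo uses flags to handle pickups capped at AmmoMax, full-clip reloads or single-round use, with printed status messages.
; All three, pickups included, require ammo remaining, and reloads deduct a whole clip from reserve regardless of rounds left.
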(event EventBeginPlay)

(event EventActorBeginOverlap
  (params (OtherActor :type Actor%20Object%20Reference)))

(event EventTick
  (params (DeltaSeconds :type Float%20%28single-precision%29)))

(fn ConstructionScript
  (|CallParentFunction)
  (Variables|Default|SetAmmoInClip (Math|Conversions|ToInteger(Byte) (Variables|Default|GetClipSize))))

(fn UpdateAmmo
  (params (Reload? :type Boolean) (AmmoPickedUp? :type Boolean) (AmountPickedUp :type Integer))
  (bind _clipsize (Variables|Default|GetClipSize))
  (bind _ammomax (Variables|Default|GetAmmoMax))
  (bind _returnvalue (Math|Conversions|ToInteger(Byte) _clipsize))
  (if (or (> (Variables|Default|GetAmmoLeft) 0) (> (Variables|Default|GetAmmoInClip) 0))
    (if AmmoPickedUp?
      (if (> (+ AmountPickedUp (Variables|Default|GetAmmoLeft)) _ammomax)
        (Variables|Default|SetAmmoLeft _ammomax)
        (Development|PrintString "Ammo Full!")
        (else
          (Variables|Default|SetAmmoLeft (+ AmountPickedUp (Variables|Default|GetAmmoLeft)))))
      (elif Reload?
        (Variables|Default|SetAmmoLeft (- (Variables|Default|GetAmmoLeft) _returnvalue))
        (Variables|Default|SetAmmoInClip _returnvalue)
        (else
          (Variables|Default|SetAmmoInClip (- (Variables|Default|GetAmmoInClip) 1)))))
    (else
      (Development|PrintString "Reload Playa"))))