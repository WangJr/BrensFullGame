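; Gravity gun weapon that, in its current form, only draws a beam toward what the player aims at and applies no force.
; The Attack input toggles a Fire flag, which Tick checks alongside combat mode.
; While both hold, it refreshes arc values and traces from the camera for pawns and physics bodies, ignoring the player.
; Each hit spawns a new beam emitter from the muzzle socket to the impact point, with debug trace drawing enabled.
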(event EventBeginPlay)

(event EventActorBeginOverlap
  (params (OtherActor :type Actor%20Object%20Reference)))

(event EventTick
  (params (DeltaSeconds :type Float%20%28single-precision%29))
  (bind _skeletalmesh (Variables|Default|GetSkeletalMesh))
  (bind _cam (Variables|Default|GetCAM))
  (bind _returnvalue (Transformation|GetSocketLocation _skeletalmesh "Muzzle"))
  (|CallParentFunction 0.0)
  (if (and (Variables|Default|GetbIsInCombatMode) (stale Input|ActionEvents|InputActionAttack _output_get))
    (CallFunction|SetArcValues)
    (bind (_outhit _returnvalue_2) (Collision|LineTraceForObjects _cam (+ _cam (* (Variables|Default|GetFWV) 1e+04)) (Utilities|Array|MakeArray "ObjectTypeQuery3" "ObjectTypeQuery4") false (Utilities|Array|MakeArray (Variables|Default|GetCurrentPlayer)) "ForDuration"))
    (if _returnvalue_2
      (bind _returnvalue_3 (Effects|SpawnEmitteratLocation "/Game/Assets/Effects/GravityBeam.GravityBeam" _returnvalue (Variables|Default|GetCRT)))
      (Class|ParticleSystemComponent|SetBeamSourcePoint _returnvalue_3 0 _returnvalue)
      (Class|ParticleSystemComponent|SetBeamTargetPoint _returnvalue_3 0 (.Location (Collision|BreakHitResult _outhit))))))

(event Input|ActionEvents|InputActionAttack
  (params (Key :type Key%20Structure :default "AnyKey"))
  (:Pressed
    (bind _output_get (Variables|Default|SetFire? true)))
  (:Released
    (Variables|Default|SetFire? false)))

(fn ConstructionScript
  (|CallParentFunction))