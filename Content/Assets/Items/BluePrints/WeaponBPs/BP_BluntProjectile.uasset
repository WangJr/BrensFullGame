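; BP_BluntProjectile is a weapon projectile that knocks characters into ragdoll on impact.
; When its HitDetect component hits a BCharacter, it enables physics simulation on that character's mesh and applies an impulse of half the projectile's velocity.
; On any hit, it spawns a BPClass actor at the projectile mesh's transform, regardless of collision, then destroys itself.
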(event OnComponentHit(HitDetect)
  (params (OtherActor :type Actor%20Object%20Reference) (OtherComp :type Primitive%20Component%20Object%20Reference) (NormalImpulse :type Vector) (Hit :type Hit%20Result%20Structure%20%28by%20ref%29))
  (bind _asbcharacter (Utilities|Casting|CastToBCharacter OtherActor)
    (:then
      (Physics|SetSimulatePhysics (Variables|/Script/Engine.Character|GetMesh _asbcharacter) true)
      (Physics|AddImpulse (Variables|/Script/Engine.Character|GetMesh _asbcharacter) (* (Transformation|GetVelocity) 0.5) "None" false))
    (:CastFailed
      _))
  (Game|SpawnActorfromClass (Variables|Default|GetBPClass) (Transformation|GetWorldTransform (Variables|Default|GetProjectileMesh)) "AlwaysSpawn" 0 0)
  (Actor|DestroyActor))

(fn ConstructionScript)