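; Knife melee weapon that damages characters with swept blade traces while an attack is active.
; Each tick it samples five points between the Hilt and Tip sockets and line-traces from their previous positions, seeded when the attack starts.
; The first character hit receives damage plus a message with bone, location and swing direction, then the attack ends.
; A separate event toggles handle collision.
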(event EventToggleCollision
  (bind _handlecollision (Variables|Default|GetHandleCollision))
  ;[1 1 1] Toggle Handle Collision for Knife
  (if (Variables|Handle|GetbExtraCollision?)
    (Collision|SetCollisionEnabled _handlecollision "QueryAndPhysics")
    (else
      (Collision|SetCollisionEnabled _handlecollision "NoCollision")))
  (Variables|Handle|SetbExtraCollision? (not (Variables|Handle|GetbExtraCollision?))))

(event EventTick
  (params (DeltaSeconds :type Float%20%28single-precision%29))
  ;[1 1 1] Run Traces Each Tick When Attack Activated
  (if (Variables|Default|GetAttack?)
    (Utilities|FlowControl|Sequence
      (:then_0
        (Utilities|FlowControl|DoOnce false :!label _label
          (:Completed
            (CallFunction|CalculateHitLocations)
            (Variables|Blade|SetOldHitLocations (Variables|Blade|GetNewHitLocations)))))
      (:then_1
        (CallFunction|CalculateHitLocations)
        (CallFunction|RunTraces)
        (Variables|Blade|SetOldHitLocations (Variables|Blade|GetNewHitLocations))))
    (else
      (goto _label Reset))))

(fn ConstructionScript
  (|CallParentFunction))

(fn CalculateHitLocations
  (bind _sitemmesh (Variables|Default|GetSItemMesh))
  (bind _returnvalue (Transformation|GetSocketLocation _sitemmesh "Hilt"))
  (bind _returnvalue_2 (Transformation|GetSocketLocation _sitemmesh "Tip"))
  (bind _returnvalue_3 (- _returnvalue_2 _returnvalue))
  (Variables|Blade|SetNewHitLocations (Utilities|Array|MakeArray _returnvalue_2 (+ (* _returnvalue_3 0.75) _returnvalue) (+ (* _returnvalue_3 0.5) _returnvalue) (+ (* _returnvalue_3 0.25) _returnvalue) _returnvalue)))

(fn RunTraces
  ;[1 0.9044 0.0479] Run Trace
  (bind _index (Utilities|FlowControl|ForLoopwithBreak 0 4 :!label _label)
    (:LoopBody
      (bind (_outhit _returnvalue) (Collision|LineTraceForObjects (Utilities|Array|Get(acopy) (Variables|Blade|GetOldHitLocations) _index) (Utilities|Array|Get(acopy) (Variables|Blade|GetNewHitLocations) _index) (LocalVariables|GetObjectsToTrace) false (Utilities|Array|MakeArray (Variables|Default|GetCurrentPlayer)) "ForDuration"))
      ;[1 1 1] Set Physics on Hit
      (if _returnvalue
        (bind _asbcharacter (Utilities|Casting|CastToBCharacter (.HitActor (Collision|BreakHitResult _outhit))))
        (if (> (Variables|/Script/BrensFullGame.BCharacter|GetCurrentHealth _asbcharacter) (Variables|Default|GetBaseDamage))
          (Variables|Default|SetImpVector (* (Math|Vector|Normalize (- (Utilities|Array|Get(acopy) (Variables|Blade|GetNewHitLocations) _index) (Utilities|Array|Get(acopy) (Variables|Blade|GetOldHitLocations) _index))) 1e+04))
          (Variables|Default|SetImpulse? false)
          (else
            (Variables|Default|SetImpVector (* (Math|Vector|Normalize (- (Utilities|Array|Get(acopy) (Variables|Blade|GetNewHitLocations) _index) (Utilities|Array|Get(acopy) (Variables|Blade|GetOldHitLocations) _index))) 1e+04))
            (Variables|Default|SetImpulse? false)))
        (Class|BCharacter|SetPlayerDamage _asbcharacter (Variables|Default|GetBaseDamage) 2 1e+01 self)
        (Class|DamageInterface|DIDamage(Message) _asbcharacter (Variables|Default|GetCurrentPlayer) (Variables|Default|GetImpulse?) (Variables|Default|GetImpVector) (.HitBoneName (Collision|BreakHitResult _outhit)) (.Location (Collision|BreakHitResult _outhit)))
        (Variables|Default|SetAttack? false)
        (goto _label Break)))))

(fn CalculateImpulse)