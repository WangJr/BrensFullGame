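; BP_DWeaponProjectile is a blunt weapon projectile that damages characters it hits.
; The construction script feeds ProjectileSpeed into the movement component's initial speed.
; On a HitDetect hit, it spawns BPClass at the mesh transform, then destroys itself.
; A hit BCharacter first gets an impulse damage message with the projectile's velocity and Spawner, plus fixed damage credited to the newly spawned actor.
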(event OnComponentHit(HitDetect)
  (params (OtherActor :type Actor%20Object%20Reference) (OtherComp :type Primitive%20Component%20Object%20Reference) (NormalImpulse :type Vector) (Hit :type Hit%20Result%20Structure%20%28by%20ref%29))
  (bind _returnvalue (Game|SpawnActorfromClass (Variables|Default|GetBPClass) (Transformation|GetWorldTransform (Variables|Default|GetProjectileMesh)) "AlwaysSpawn" 0 0))
  (bind _asbcharacter (Utilities|Casting|CastToBCharacter OtherActor)
    (:then
      (Class|DamageInterface|DIDamage(Message) _asbcharacter (Variables|Default|GetSpawner) true (Transformation|GetVelocity) "None" "0, 0, 0")
      (Class|BCharacter|SetPlayerDamage _asbcharacter 10 0 0.0 _returnvalue))
    (:CastFailed
      _))
  (Actor|DestroyActor))

(fn ConstructionScript
  (Variables|/Script/Engine.ProjectileMovementComponent|SetInitialSpeed (Variables|Default|GetProjectileMovement) (Variables|Default|GetProjectileSpeed)))