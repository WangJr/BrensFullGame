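; BP_DWProjectile is a weapon projectile that rolls its mesh in flight and knocks down characters it hits.
; Tick advances a counter that wraps to -1 outside the -1 to 1 range, using its arcsine in degrees as mesh roll.
; On a HitDetect hit, a BCharacter's mesh starts simulating physics and receives an impulse from projectile velocity.
; Any hit spawns a BPClass actor at the mesh transform and destroys the projectile.
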(event OnComponentHit(HitDetect)
  (params (OtherActor :type Actor%20Object%20Reference) (OtherComp :type Primitive%20Component%20Object%20Reference) (NormalImpulse :type Vector) (Hit :type Hit%20Result%20Structure%20%28by%20ref%29))
  (bind _asbcharacter (Utilities|Casting|CastToBCharacter OtherActor)
    (:then
      (Physics|SetSimulatePhysics (Variables|/Script/Engine.Character|GetMesh _asbcharacter) true)
      (Physics|AddImpulse (Variables|/Script/Engine.Character|GetMesh _asbcharacter) (* (Transformation|GetVelocity) 0.5) "None" false))
    (:CastFailed
      _))
  (Game|SpawnActorfromClass (Variables|Default|GetBPClass) (Transformation|GetWorldTransform (Variables|Default|GetProjectileMesh)) "AlwaysSpawn" 0 0)
  (Actor|DestroyActor))

(event EventTick
  (params (DeltaSeconds :type Float%20%28single-precision%29))
  (bind _projectilemesh (Variables|Default|GetProjectileMesh))
  (bind _relativerotation (Variables|/Script/Engine.SceneComponent|GetRelativeRotation _projectilemesh))
  (bind (_roll _pitch _yaw) (Math|Rotator|BreakRotator _relativerotation))
  (bind _output_get (Variables|Default|SetCount (+ (* DeltaSeconds (Math|Float|MakeLiteralFloat 5.0)) (Variables|Default|GetCount))))
  (if (Math|Float|InRange(Float) _output_get -1.0 1.0)
    (Transformation|SetRelativeRotation _projectilemesh (Math|Rotator|MakeRotator (Class|KismetMathLibrary|DegAsin _output_get) _pitch _yaw) false false)
    (else
      (Variables|Default|SetCount -1.0))))

(fn ConstructionScript)