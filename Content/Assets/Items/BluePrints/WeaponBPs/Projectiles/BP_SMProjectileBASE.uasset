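; BP_SMProjectileBASE is a base weapon projectile Blueprint that moves via a ProjectileMovement component and removes itself after a set lifetime.
; Its construction script copies the Speed variable into the component's initial speed and Size into ItemSize.
; Tick accumulates delta time in a Timer and destroys the actor once it reaches Lifetime.
; The graphs contain no hit or damage logic, and the overlap event is an empty placeholder.
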(event Collision|EventActorBeginOverlap
  (params (OtherActor :type Actor%20Object%20Reference)))

(event EventTick
  (params (DeltaSeconds :type Float%20%28single-precision%29))
  (bind _output_get (Variables|Default|SetTimer (+ (* DeltaSeconds (Math|Float|MakeLiteralFloat 1.0)) (Variables|Default|GetTimer))))
  (if (>= _output_get (Variables|Default|GetLifetime))
    (Actor|DestroyActor)))

(fn ConstructionScript
  (Variables|/Script/Engine.ProjectileMovementComponent|SetInitialSpeed (Variables|Default|GetProjectileMovement) (Variables|Default|GetSpeed))
  (Variables|Default|SetItemSize (Variables|Default|GetSize)))