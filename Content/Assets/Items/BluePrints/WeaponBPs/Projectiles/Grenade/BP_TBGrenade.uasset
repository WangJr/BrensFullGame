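; Time-dilation grenade projectile that explodes after a two-second Tick-counted fuse, then destroys itself.
; Detonation spawns an explosion, halves global time and sets all BCharacters to double custom dilation, offsetting the slowdown.
; A sphere trace damages and launches nearby characters, resetting their dilation so they stay slowed, and pushes other physics bodies.
; It flags every BCharacter with TD and does not restore global time itself.
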(event EventBeginPlay)

(event Collision|EventActorBeginOverlap
  (params (OtherActor :type Actor%20Object%20Reference)))

(event EventTick
  (params (DeltaSeconds :type Float%20%28single-precision%29))
  (bind _sphere (Variables|Default|GetSphere))
  (bind _returnvalue (Transformation|GetWorldLocation _sphere))
  (bind _output_get (Variables|Default|SetCount (+ (* DeltaSeconds (Math|Float|MakeLiteralFloat 1.0)) (Variables|Default|GetCount))))
  (if (>= _output_get 2.0)
    (Rendering|ToggleVisibility (Variables|Default|GetStaticMesh) false)
    (bind _returnvalue_2 (Effects|SpawnEmitteratLocation "/Game/StarterContent/Particles/P_Explosion.P_Explosion" (Transformation|GetWorldLocation _sphere)))
    (Transformation|SetWorldScale3D _returnvalue_2 "5.000000,5.000000,5.000000")
    (bind _outactors (Actor|GetAllActorsOfClass "/Script/BrensFullGame.BCharacter"))
    (for _array_element _outactors
      (Variables|/Script/BrensFullGame.BCharacter|SetTD _array_element true)
      (Variables|/Script/Engine.Actor|SetCustomTimeDilation _array_element 2.0))
    (Utilities|Time|SetGlobalTimeDilation 0.5)
    (Variables|/Script/Engine.Actor|SetCustomTimeDilation (Variables|Default|GetCurrentPlayer) 2.0)
    (bind (_outhits _returnvalue_3) (Collision|MultiSphereTraceForObjects _returnvalue (+ _returnvalue "0, 0,5.000000") 5e+02 (Utilities|Array|MakeArray "ObjectTypeQuery4" "ObjectTypeQuery3") false (Variables|Default|GetActorsToIgnore) "None"))
    (if _returnvalue_3
      (for _array_element_2 _outhits
        (Utilities|Array|Add (Variables|Default|GetActorsToIgnore) (.HitActor (Collision|BreakHitResult _array_element_2)))
        (bind _asbcharacter (Utilities|Casting|CastToBCharacter (.HitActor (Collision|BreakHitResult _array_element_2)))
          (:then
            (Class|BCharacter|SetPlayerDamage _asbcharacter 5e+01 0 0.0 self)
            (Class|DamageInterface|DIDamage(Message) _asbcharacter (Variables|Default|GetCurrentPlayer) true (Math|Vector|MakeVector (.X (Math|Vector|BreakVector (* (Math|Vector|Normalize (- (Transformation|GetActorLocation (.HitActor (Collision|BreakHitResult _array_element_2))) (Transformation|GetWorldLocation (Variables|Default|GetSphere)))) 2e+03))) (.Y (Math|Vector|BreakVector (* (Math|Vector|Normalize (- (Transformation|GetActorLocation (.HitActor (Collision|BreakHitResult _array_element_2))) (Transformation|GetWorldLocation (Variables|Default|GetSphere)))) 2e+03))) 2e+03) (.HitBoneName (Collision|BreakHitResult _array_element_2)) (.Location (Collision|BreakHitResult _array_element_2)))
            (Variables|/Script/Engine.Actor|SetCustomTimeDilation _asbcharacter 1.0))
          (:CastFailed
            (Physics|AddImpulseatLocation (.HitComponent (Collision|BreakHitResult _array_element_2)) (Math|Vector|MakeVector (.X (Math|Vector|BreakVector (* (Math|Vector|Normalize (- (Transformation|GetActorLocation (.HitActor (Collision|BreakHitResult _array_element_2))) (Transformation|GetWorldLocation (Variables|Default|GetSphere)))) 2e+03))) (.Y (Math|Vector|BreakVector (* (Math|Vector|Normalize (- (Transformation|GetActorLocation (.HitActor (Collision|BreakHitResult _array_element_2))) (Transformation|GetWorldLocation (Variables|Default|GetSphere)))) 2e+03))) 2e+03) (.Location (Collision|BreakHitResult _array_element_2)) (.HitBoneName (Collision|BreakHitResult _array_element_2)))))))
    (Actor|DestroyActor)))

(fn ConstructionScript)