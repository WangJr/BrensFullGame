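; BP_BasicGrenade is a timed grenade projectile that explodes 2.5 seconds after spawning, then destroys itself.
; Tick accumulates the fuse time, then hides the mesh, spawns a scaled-up explosion emitter and sphere-traces for pawns and physics bodies.
; BCharacter hits take flat damage and receive a damage message carrying the sender, outward impulse and bone.
; Other hits get an outward impulse with a fixed upward kick.
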(event EventBeginPlay)

(event EventActorBeginOverlap
  (params (OtherActor :type Actor%20Object%20Reference)))

(event EventTick
  (params (DeltaSeconds :type Float%20%28single-precision%29))
  (bind _sphere (Variables|Default|GetSphere))
  (bind _returnvalue (Transformation|GetWorldLocation _sphere))
  (bind _output_get (Variables|Default|SetCount (+ (* DeltaSeconds (Math|Float|MakeLiteralFloat 1.0)) (Variables|Default|GetCount))))
  (if (>= _output_get 2.5)
    (Rendering|ToggleVisibility (Variables|Default|GetStaticMesh) false)
    (bind _returnvalue_2 (Effects|SpawnEmitteratLocation "/Game/StarterContent/Particles/P_Explosion.P_Explosion" (Transformation|GetWorldLocation (Variables|Default|GetSphere))))
    (Transformation|SetWorldScale3D _returnvalue_2 "5.000000,5.000000,5.000000")
    (bind (_outhits _returnvalue_3) (Collision|MultiSphereTraceForObjects _returnvalue (+ _returnvalue "0, 0,5.000000") 5e+02 (Utilities|Array|MakeArray "ObjectTypeQuery4" "ObjectTypeQuery3") false 0 "None"))
    (if _returnvalue_3
      (for _array_element _outhits
        (bind _asbcharacter (Utilities|Casting|CastToBCharacter (.HitActor (Collision|BreakHitResult _array_element)))
          (:then
            (Class|BCharacter|SetPlayerDamage _asbcharacter 120 0 0.0)
            (Class|DamageInterface|DIDamage(Message) _asbcharacter (Variables|Default|GetCurrentPlayer) true (* (Math|Vector|Normalize (- (Transformation|GetActorLocation (.HitActor (Collision|BreakHitResult _array_element))) (Transformation|GetWorldLocation (Variables|Default|GetSphere)))) 2e+03) (.HitBoneName (Collision|BreakHitResult _array_element)) "0, 0, 0"))
          (:CastFailed
            (Physics|AddImpulseatLocation (.HitComponent (Collision|BreakHitResult _array_element)) (Math|Vector|MakeVector (.X (Math|Vector|BreakVector (* (Math|Vector|Normalize (- (Transformation|GetActorLocation (.HitActor (Collision|BreakHitResult _array_element))) (Transformation|GetWorldLocation (Variables|Default|GetSphere)))) 2e+03))) (.Y (Math|Vector|BreakVector (* (Math|Vector|Normalize (- (Transformation|GetActorLocation (.HitActor (Collision|BreakHitResult _array_element))) (Transformation|GetWorldLocation (Variables|Default|GetSphere)))) 2e+03))) 4e+03) (.Location (Collision|BreakHitResult _array_element)) (.HitBoneName (Collision|BreakHitResult _array_element)))))))
    (Actor|DestroyActor)))

(fn ConstructionScript)