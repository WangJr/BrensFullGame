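; BP_DWeaponProjectile is a weapon projectile that damages characters on impact and leaves a spawned actor where it lands.
; When HitDetect hits anything except the Spawner, a BCharacter target receives an impulse damage message carrying the projectile's velocity, plus fixed damage.
; It then spawns BPClass at the mesh transform and destroys itself.
; The damage call's Hitter references that spawned actor before the spawn runs.
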(event OnComponentHit(HitDetect)
  (params (OtherActor :type Actor%20Object%20Reference) (OtherComp :type Primitive%20Component%20Object%20Reference) (NormalImpulse :type Vector) (Hit :type Hit%20Result%20Structure%20%28by%20ref%29))
  (bind _spawner (Variables|Default|GetSpawner))
  (if (!= OtherActor _spawner)
    (bind _asbcharacter (Utilities|Casting|CastToBCharacter OtherActor)
      (:then
        (Class|DamageInterface|DIDamage(Message) _asbcharacter _spawner true (Transformation|GetVelocity) "None" (Transformation|GetActorLocation OtherActor))
        (Class|BCharacter|SetPlayerDamage _asbcharacter 10 0 0.0 (stale _returnvalue)))
      (:CastFailed
        _))
    (bind _returnvalue (Game|SpawnActorfromClass (Variables|Default|GetBPClass) (Transformation|GetWorldTransform (Variables|Default|GetProjectileMesh)) "AlwaysSpawn" 0 0))
    (Actor|DestroyActor)))

(fn ConstructionScript)