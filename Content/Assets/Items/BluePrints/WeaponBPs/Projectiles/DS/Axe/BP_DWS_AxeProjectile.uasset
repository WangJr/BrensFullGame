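; Thrown axe projectile that spins in flight and resolves as either a sharp or blunt hit.
; Each tick it traces between previous and current mesh socket positions, with blade traces running only during part of the rotation.
; A blade hit spawns a non-physical axe stuck at impact, attached to any struck character's bone; a blunt hit spawns a physics-simulated one.
; Struck characters take damage by hit type, then the projectile destroys itself.
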(event EventTick
  (params (DeltaSeconds :type Float%20%28single-precision%29))
  (bind _projectilemesh (Variables|Default|GetProjectileMesh))
  (bind _relativerotation (Variables|/Script/Engine.SceneComponent|GetRelativeRotation _projectilemesh))
  (bind (_roll _pitch _yaw) (Math|Rotator|BreakRotator _relativerotation))
  ;[1 1 1] Set Projectile Rotation based on Spawn Time
  (bind _output_get (Variables|Default|SetAngle_0 (+ (* DeltaSeconds (Variables|Default|GetDegPerSec)) (Variables|Default|GetAngle_0))))
  (if (Math|Float|InRange(Float) (+ (* DeltaSeconds (Variables|Default|GetDegPerSec)) (Variables|Default|GetAngle_0)) 0.0 3.6e+02 true false)
    _
    (else
      (Variables|Default|SetAngle_0 0.0)))
  (Transformation|SetRelativeRotation _projectilemesh (Math|Rotator|MakeRotator _output_get _pitch _yaw) false false)
  (Development|PrintString (Utilities|String|ToString(Float) (Math|Vector|VectorLength (Transformation|GetVelocity))))
  ;[1 1 1] Check If Blade is in a Position to do Damage (now = 0-90, future = 330-60ish
  (bind _output_get_2 (Variables|Default|Set90? (Math|Float|InRange(Float) (Variables|Default|GetAngle_0) 0.0 9e+01 true false)))
  (if _output_get_2
    (Utilities|FlowControl|Sequence
      (:then_0
        ;[1 1 1] Intilalize Old Hit Locations when Blade can once again do Damage
        (Utilities|FlowControl|DoOnce false :!label _label
          (:Completed
            (Utilities|Array|Clear (Variables|Default|GetOHL))
            (CallFunction|CalculateNHL)
            (Variables|Default|SetOHL (Variables|Default|GetNHL))
            (Variables|Default|SetOld%20Transform (Transformation|GetWorldTransform (Variables|Default|GetProjectileMesh))))))
      (:then_1
        ;[1 1 1] Calculate New Hit Locations and Run Traces for Sharp Hit
        (CallFunction|CalculateNHL)
        (CallFunction|RunTraces)
        ;[1 1 1] Check if Sharp Hit was Success
        (if (Variables|Default|GetAHit?) :!label _label_2
          ;[1 1 1] If Hit Destroy Projectile
          (bind _asbcharacter (Utilities|Casting|CastToBCharacter (Variables|Default|GetHitActor) :!label _label_3)
            (:then
              (if (Variables|Default|GetAHit?)
                (Variables|Default|SetDT 1)
                (Variables|Default|SetDB 35)
                (else
                  (Variables|Default|SetDT 0)
                  (Variables|Default|SetDB 5)))
              (Class|BCharacter|SetPlayerDamage _asbcharacter (Variables|Default|GetDB) (Variables|Default|GetDT) 0.0 (stale _returnvalue_2))
              (Class|DamageInterface|DIDamage(Message) _asbcharacter (Variables|Default|GetSpawner) true (* (Transformation|GetVelocity) 1e+03) (Variables|Default|GetHitBone) "0, 0, 0"))
            (:CastFailed
              _))
          (Actor|DestroyActor)
          (else
            ;[1 1 1] Run Trace for Blunt Hit
            (bind (_outhit _returnvalue) (Collision|LineTraceForObjects (Utilities|Array|Get(acopy) (Variables|Default|GetOHL) 3) (Utilities|Array|Get(acopy) (Variables|Default|GetNHL) 3) (Utilities|Array|MakeArray "ObjectTypeQuery3" "ObjectTypeQuery1") false (Utilities|Array|MakeArray (Variables|Default|GetSpawner)) "None"))
            (if _returnvalue
              (bind _returnvalue_2 (Game|SpawnActorfromClass (Variables|Default|GetBPClass) (Variables|Default|GetOld%20Transform) "AdjustIfPossibleButAlwaysSpawn" 0 0))
              (Variables|Default|SetHitActor (.HitActor (Collision|BreakHitResult _outhit)))
              (Physics|SetSimulatePhysics (Variables|/Game/Assets/Items/BluePrints/BP_DItem.BP_DItem_C|GetSkeletalMesh _returnvalue_2) true)
              (Variables|/Script/BrensFullGame.Item|SetItemSize _returnvalue_2 (Variables|Default|GetBPSize))
              (goto _label_3)
              (else
                ;[1 1 1] If No Successful Hits, Set Old Values and Reset DoOnceGate
                (Variables|Default|SetOHL (Variables|Default|GetNHL))
                (Variables|Default|SetOld%20Transform (Transformation|GetWorldTransform (Variables|Default|GetProjectileMesh)))
                (if (not (Variables|Default|Get90?))
                  (goto _label Reset))))))))
    (else
      ;[1 1 1] If Angle no in Range, set NHL so you can check for Blunt Hit
      (CallFunction|CalculateNHL)
      (goto _label_2))))

(fn ConstructionScript
  (|CallParentFunction)
  (Variables|Default|SetDegPerSec 1.2e+03))

(fn CalculateNHL
  (Utilities|Array|Clear (Variables|Default|GetNHL))
  (for _array_element (Variables|Default|GetHitNames)
    (Utilities|Array|Add (Variables|Default|GetNHL) (Transformation|GetSocketLocation (Variables|Default|GetProjectileMesh) _array_element)))
  (return))

(fn RunTraces
  (bind _old_transform (Variables|Default|GetOld%20Transform))
  (bind (_location _rotation _scale) (Math|Transform|BreakTransform _old_transform))
  (bind _index (Utilities|FlowControl|ForLoopwithBreak 0 2 :!label _label)
    (:LoopBody
      (bind (_outhit _returnvalue) (Collision|LineTraceForObjects (Utilities|Array|Get(acopy) (Variables|Default|GetOHL) _index) (Utilities|Array|Get(acopy) (Variables|Default|GetNHL) _index) (Utilities|Array|MakeArray "ObjectTypeQuery3" "ObjectTypeQuery1") false (Utilities|Array|MakeArray (Variables|Default|GetSpawner)) "None"))
      (if _returnvalue
        (Variables|Default|SetHitActor (.HitActor (Collision|BreakHitResult _outhit)))
        (Variables|Default|SetHitBone (.HitBoneName (Collision|BreakHitResult _outhit)))
        (bind _returnvalue_2 (Game|SpawnActorfromClass (Variables|Default|GetBPClass) (Math|Transform|MakeTransform (+ _location (- (.Location (Collision|BreakHitResult _outhit)) (Utilities|Array|Get(acopy) (Variables|Default|GetOHL) _index))) (Transformation|GetWorldRotation (Variables|Default|GetProjectileMesh)) _scale) "AlwaysSpawn" 0 0))
        (Physics|SetSimulatePhysics (Variables|/Game/Assets/Items/BluePrints/BP_DItem.BP_DItem_C|GetSkeletalMesh _returnvalue_2) false)
        (Collision|SetCollisionEnabled (Variables|/Game/Assets/Items/BluePrints/BP_DItem.BP_DItem_C|GetSkeletalMesh _returnvalue_2) "NoCollision")
        (Variables|/Script/BrensFullGame.Item|SetItemSize _returnvalue_2 (Variables|Default|GetBPSize))
        (Variables|Default|SetAHit? true)
        (bind _asbcharacter (Utilities|Casting|CastToBCharacter (Variables|Default|GetHitActor))
          (:then
            (Class|Actor|AttachRootComponentto _returnvalue_2 (Variables|/Script/Engine.Character|GetMesh _asbcharacter) (Variables|Default|GetHitBone) "KeepWorldPosition" true)
            (goto _label Break))
          (:CastFailed
            (goto _label Break)))))))