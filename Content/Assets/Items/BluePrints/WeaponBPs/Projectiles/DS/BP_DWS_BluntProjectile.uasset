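; Blunt weapon projectile that spins in flight and turns back into a spawned item on impact.
; Each tick it rolls its mesh, prints its speed, and sphere-traces at HitDetect for pawns other than the Spawner, then for static world geometry.
; Either hit spawns BPClass at the mesh transform with BPSize and destroys the projectile.
; Character hits also deal fixed damage credited to the spawned item and send a velocity-scaled impulse.
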(event EventTick
  (params (DeltaSeconds :type Float%20%28single-precision%29))
  (bind _hitdetect (Variables|Default|GetHitDetect))
  (bind _projectilemesh (Variables|Default|GetProjectileMesh))
  (bind _returnvalue (Transformation|GetWorldLocation _hitdetect))
  (bind _relativerotation (Variables|/Script/Engine.SceneComponent|GetRelativeRotation _projectilemesh))
  (bind (_roll _pitch _yaw) (Math|Rotator|BreakRotator _relativerotation))
  (bind _returnvalue_2 (+ _returnvalue "1.000000, 0,0.000000"))
  ;[1 1 1] Rotation Control
  (Development|PrintString 0 (Utilities|String|ToString(Float) (Math|Vector|VectorLength (Transformation|GetVelocity))))
  (bind _output_get (Variables|Default|SetAngle (+ (* DeltaSeconds (Variables|Default|GetDegPerSec)) (Variables|Default|GetAngle))))
  (if (Math|Float|InRange(Float) _output_get 0.0 3.6e+02)
    (Transformation|SetRelativeRotation _projectilemesh (Math|Rotator|MakeRotator _output_get _pitch _yaw) false false)
    (else
      (Variables|Default|SetAngle 0.0)))
  ;[1 1 1] Sphere Trace for Pawn
  (bind (_outhit _returnvalue_3) (Collision|SphereTraceForObjects 0 _returnvalue _returnvalue_2 32.0 (Utilities|Array|MakeArray "ObjectTypeQuery3") false (Utilities|Array|MakeArray (Variables|Default|GetSpawner)) "None"))
  ;[1 1 1] Set if Player/AI is hit
  (bind _output_get_2 (Variables|Default|SetPlayerHit? _returnvalue_3))
  (if _output_get_2
    ;[1 1 1] If Hit, Spawn BP of Spawner Class
    (bind _returnvalue_4 (Game|SpawnActorfromClass (Variables|Default|GetBPClass) (Transformation|GetWorldTransform (Variables|Default|GetProjectileMesh)) "AdjustIfPossibleButAlwaysSpawn" 0 0 :!label _label))
    (Variables|/Script/BrensFullGame.Item|SetItemSize _returnvalue_4 (Variables|Default|GetBPSize))
    (if (Variables|Default|GetPlayerHit?)
      ;[1 1 1] If Player/AI Hit, Apply Blunt Damage
      (bind _asbcharacter (Utilities|Casting|CastToBCharacter (.HitActor (Collision|BreakHitResult _outhit))))
      (Class|BCharacter|SetPlayerDamage _asbcharacter 34.0 0 0.0 _returnvalue_4)
      (Class|DamageInterface|DIDamage(Message) _asbcharacter (Variables|Default|GetSpawner) true (* (Transformation|GetVelocity) 5e+01) "None" "0, 0, 0"))
    (Actor|DestroyActor)
    (else
      ;[1 1 1] Sphere Trace for World Static
      (bind _returnvalue_5 (Collision|SphereTraceForObjects 0 _returnvalue _returnvalue_2 32.0 (Utilities|Array|MakeArray "ObjectTypeQuery1") false 0 "None"))
      (if _returnvalue_5
        (goto _label)))))

(fn ConstructionScript
  (|CallParentFunction))