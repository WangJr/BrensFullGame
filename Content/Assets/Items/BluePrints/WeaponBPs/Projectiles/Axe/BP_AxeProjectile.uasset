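; Thrown axe projectile that rolls in flight and turns into a spawned BPClass actor on impact.
; Each Tick sweeps mesh roll through a looping arcsine counter and line-traces between socket pairs, ignoring the Spawner, with debug drawing.
; A Back-Front hit freezes the spawned actor, attaching it to the struck bone on BCharacters.
; Otherwise, a Tip-Hilt hit spawns it unfrozen; either hit destroys the projectile.
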(event EventBeginPlay)

(event EventActorBeginOverlap
  (params (OtherActor :type Actor%20Object%20Reference)))

(event EventTick
  (params (DeltaSeconds :type Float%20%28single-precision%29))
  (bind _projectilemesh (Variables|Default|GetProjectileMesh))
  (bind _projectilemesh_2 (Variables|Default|GetProjectileMesh))
  (bind _relativerotation (Variables|/Script/Engine.SceneComponent|GetRelativeRotation _projectilemesh))
  (bind (_roll _pitch _yaw) (Math|Rotator|BreakRotator _relativerotation))
  (bind _output_get (Variables|Default|SetCount (+ (* DeltaSeconds (Math|Float|MakeLiteralFloat 5.0)) (Variables|Default|GetCount))))
  (if (Math|Float|InRange(Float) _output_get -1.0 1.0)
    (Transformation|SetRelativeRotation _projectilemesh (Math|Rotator|MakeRotator (Class|KismetMathLibrary|DegAsin _output_get) _pitch _yaw) false false)
    (else
      (Variables|Default|SetCount -1.0)))
  (bind (_outhit _returnvalue) (Collision|LineTraceForObjects (Transformation|GetSocketLocation _projectilemesh_2 "Back") (Transformation|GetSocketLocation _projectilemesh_2 "Front") (Utilities|Array|MakeArray "ObjectTypeQuery3" "ObjectTypeQuery1") false (Utilities|Array|MakeArray (Variables|Default|GetSpawner)) "ForDuration"))
  (if _returnvalue
    (bind _returnvalue_2 (Game|SpawnActorfromClass (Variables|Default|GetBPClass) (Transformation|GetWorldTransform (Variables|Default|GetProjectileMesh)) "AlwaysSpawn" 0 0))
    (Physics|SetSimulatePhysics (Variables|/Game/Assets/Items/BluePrints/BP_DItem.BP_DItem_C|GetSkeletalMesh _returnvalue_2) false)
    (Collision|SetCollisionEnabled (Variables|/Game/Assets/Items/BluePrints/BP_DItem.BP_DItem_C|GetSkeletalMesh _returnvalue_2) "NoCollision")
    (bind _asbcharacter (Utilities|Casting|CastToBCharacter (.HitActor (Collision|BreakHitResult _outhit)))
      (:then
        (Class|Actor|AttachRootComponentto _returnvalue_2 (Variables|/Script/Engine.Character|GetMesh _asbcharacter) (.HitBoneName (Collision|BreakHitResult _outhit)) "KeepWorldPosition" true))
      (:CastFailed
        _))
    (Actor|DestroyActor :!label _label)
    (else
      (bind (_outhit_2 _returnvalue_3) (Collision|LineTraceForObjects (Transformation|GetSocketLocation _projectilemesh_2 "Tip") (Transformation|GetSocketLocation _projectilemesh_2 "Hilt") (Utilities|Array|MakeArray "ObjectTypeQuery3" "ObjectTypeQuery1") false (Utilities|Array|MakeArray (Variables|Default|GetSpawner)) "ForDuration"))
      (if _returnvalue_3
        (Game|SpawnActorfromClass (Variables|Default|GetBPClass) (Transformation|GetWorldTransform (Variables|Default|GetProjectileMesh)) "AdjustIfPossibleButAlwaysSpawn" 0 0)
        (goto _label)))))

(fn ConstructionScript
  (|CallParentFunction))