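; BP_DWeapon is a weapon actor that players pick up, drop and attack with.
; Overlapping a character enables the weapon's input, and F alternates between attaching it to the WeaponHolster socket and dropping it, toggling collision and physics.
; Attack input drives the player's animation instance and attacking flag.
; In combat mode, gun-type items cast to BP_DGun to spawn muzzle bullets or reload when empty.
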(event OnComponentBeginOverlap(Overlapdetect)
  (params (OtherActor :type Actor%20Object%20Reference) (OtherComp :type Primitive%20Component%20Object%20Reference) (OtherBodyIndex :type Integer) (bFromSweep :type Boolean) (SweepResult :type Hit%20Result%20Structure%20%28by%20ref%29))
  ;[1 1 1] Enable/Disable Input
  (Utilities|Casting|CastToBCharacterClass (Utilities|GetClass OtherActor))
  (Variables|Default|SetCurrentPlayer OtherActor)
  (Development|PrintString 0 "ENTERING!!!!!")
  (Input|EnableInput (Game|GetPlayerController 0)))

(event OnComponentEndOverlap(Overlapdetect)
  (params (OtherActor :type Actor%20Object%20Reference) (OtherComp :type Primitive%20Component%20Object%20Reference) (OtherBodyIndex :type Integer))
  ;[1 1 1] Enable/Disable Input
  (Utilities|Casting|CastToBCharacterClass (Utilities|GetClass OtherActor))
  (Development|PrintString 0 "Exiting!!!!!!!")
  (Input|DisableInput (Game|GetPlayerController 0)))

(event Input|ActionEvents|InputActionAttack
  (params (Key :type Key%20Structure :default "AnyKey"))
  (bind _currentplayer (Variables|Default|GetCurrentPlayer))
  ;[1 1 1] Attack
  (:Pressed
    (bind _asbp_bplayer (Utilities|Casting|CastToBP_BPlayer _currentplayer))
    (if (Variables|/Script/BrensFullGame.BCharacter|GetIsItemHeld _asbp_bplayer)
      (Class|CombatModeInterface|AttackStart(Message) (Components|SkeletalMesh|GetAnimInstance (Variables|/Script/Engine.Character|GetMesh _asbp_bplayer)))
      (Variables|/Game/Assets/Characters/BP_BPlayer.BP_BPlayer_C|SetAttacking? _asbp_bplayer true)
      (Development|PrintString "Attacking")
      (if (and (Variables|/Game/Assets/Characters/BP_BPlayer.BP_BPlayer_C|GetCombatMode? _asbp_bplayer) (== (Variables|/Script/BrensFullGame.BCharacter|GetItemType _asbp_bplayer) 2))
        (bind _asbp_dgun (Utilities|Casting|CastToBP_DGun (Variables|/Script/BrensFullGame.BCharacter|GetHeldItem _asbp_bplayer)))
        (if (> (Variables|BP_DWeapon_C|GetAmmoInClip _asbp_dgun) 0)
          (Game|SpawnActorfromClass "/Game/Assets/Items/BluePrints/WeaponBPs/DynamicWeapons/RegularBullet.RegularBullet_C" (Transformation|GetSocketTransform (Variables|BP_DWeapon_C|GetSkeletalMesh _asbp_dgun) "Muzzle" "RTS_World") "AdjustIfPossibleButDontSpawnIfColliding" 0 0)
          (Default|UpdateAmmo _asbp_dgun false false)
          (else
            (Default|UpdateAmmo _asbp_dgun true false)
            (Utilities|FlowControl|Delay 0.2))))))
  (:Released
    (bind _asbp_bplayer_2 (Utilities|Casting|CastToBP_BPlayer _currentplayer))
    (Variables|/Game/Assets/Characters/BP_BPlayer.BP_BPlayer_C|SetAttacking? _asbp_bplayer_2 false)
    (Class|CombatModeInterface|AttackEnd(Message) (Components|SkeletalMesh|GetAnimInstance (Variables|/Script/Engine.Character|GetMesh _asbp_bplayer)))
    (Development|PrintString "Stoppinglo")))

(event Input|KeyboardEvents|F
  (params (Key :type Key%20Structure :default "AnyKey"))
  (bind _returnvalue (Game|GetPlayerController 0))
  (bind _currentplayer (Variables|Default|GetCurrentPlayer))
  (bind _itemtype (Variables|Default|GetItemType))
  ;[1 1 1] Pickup
  (:Pressed
    (bind _counter (Utilities|FlowControl|DoN 2 :!label _label)
      (:Exit
        (switch int _counter
          (:1
            (bind _asbcharacter (Utilities|Casting|CastToBCharacter _currentplayer))
            (if (not (Variables|/Script/BrensFullGame.BCharacter|GetIsItemHeld _asbcharacter))
              (CallFunction|SetCollision false)
              (Class|Actor|AttachRootComponentto (Variables|/Script/Engine.Character|GetMesh _asbcharacter) "WeaponHolster" "SnapToTarget" true)
              (Class|BCharacter|SetValues _asbcharacter self _itemtype true)
              (Input|EnableInput _returnvalue)
              (if (== _itemtype 2)
                (Variables|Ammo|SetbGun? true)
                (else
                  (Variables|Ammo|SetbGun? false)))))
          (:2
            (bind _asbp_bplayer (Utilities|Casting|CastToBP_BPlayer _currentplayer))
            (Development|PrintString "Input is on Item")
            (Class|Actor|DetachRootComponentfromParent true)
            (Utilities|FlowControl|Delay 0.2)
            (CallFunction|SetCollision true)
            (Default|JumpOutOfCombatMode _asbp_bplayer)
            (Input|DisableInput _returnvalue)
            (goto _label Reset)))))))

(fn ConstructionScript)

(fn SetCollision
  (params (On? :type Boolean))
  (bind _overlapdetect (Variables|Default|GetOverlapDetect))
  (bind _skeletalmesh (Variables|Default|GetSkeletalMesh))
  (if On?
    (Collision|SetCollisionEnabled _overlapdetect "QueryAndPhysics")
    (Collision|SetCollisionEnabled _skeletalmesh "QueryAndPhysics")
    (else
      (Collision|SetCollisionEnabled _overlapdetect "NoCollision")
      (Collision|SetCollisionEnabled _skeletalmesh "NoCollision")))
  (Physics|SetSimulatePhysics _skeletalmesh On?))