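; Test projectile that impales a character and pins it to static world geometry, using two overlap detectors.
; HitDetect overlapping a BCharacter line-traces to HitDetect2, enables physics on the hit component and constrains the struck bone to the projectile.
; HitDetect2 touching WorldStatic stops movement and swaps the projectile for a spawned, non-simulating item, whose Impalor constraint takes over the stored mesh and bone.
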(event OnComponentBeginOverlap(HitDetect2)
  (params (OtherActor :type Actor%20Object%20Reference) (OtherComp :type Primitive%20Component%20Object%20Reference) (OtherBodyIndex :type Integer) (bFromSweep :type Boolean) (SweepResult :type Hit%20Result%20Structure%20%28by%20ref%29))
  (bind _projectilemovement (Variables|Default|GetProjectileMovement))
  ;[1 1 1] Basic Collision Mechanics
  (if (Utilities|Enum|Equal(Enum) (Collision|GetCollisionObjectType OtherComp) "ECC_WorldStatic")
    (Utilities|FlowControl|DoOnce false
      (:Completed
        (Components|Movement|StopMovementImmediately _projectilemovement)
        (Variables|/Script/Engine.ProjectileMovementComponent|SetbRotationFollowsVelocity _projectilemovement false)
        (bind _returnvalue (Game|SpawnActorfromClass (Variables|Default|GetBPClass) (Transformation|GetWorldTransform (Variables|Default|GetProjectileMesh)) "AlwaysSpawn" 0 0))
        (Physics|SetSimulatePhysics (Variables|/Script/BrensFullGame.SItem|GetSItemMesh _returnvalue) false)
        (Class|PhysicsConstraintComponent|SetConstrainedComponents (Variables|Default|GetPhysicsConstraint) 0 "None" 0 "None")
        (Transformation|SetWorldLocation (Variables|/Game/Assets/Items/BluePrints/WeaponBPs/BP_SWeapon.BP_SWeapon_C|GetImpalLocation _returnvalue) (Transformation|GetWorldLocation (Variables|Default|GetHitDetect)) false true)
        (Class|PhysicsConstraintComponent|SetConstrainedComponents (Variables|/Game/Assets/Items/BluePrints/WeaponBPs/BP_SWeapon.BP_SWeapon_C|GetImpalor _returnvalue) (Variables|/Game/Assets/Items/BluePrints/WeaponBPs/BP_SWeapon.BP_SWeapon_C|GetImpalLocation _returnvalue) "None" (Variables|Default|GetHitMesh) (Variables|Default|GetHitBone))
        (Class|PhysicsConstraintComponent|SetDisableCollision (Variables|/Game/Assets/Items/BluePrints/WeaponBPs/BP_SWeapon.BP_SWeapon_C|GetImpalor _returnvalue) true)
        (Actor|DestroyActor)
        (Variables|/Game/Assets/Items/BluePrints/WeaponBPs/BP_SWeapon.BP_SWeapon_C|SetbImpaled? _returnvalue true)))))

(event OnComponentBeginOverlap(HitDetect)
  (params (OtherActor :type Actor%20Object%20Reference) (OtherComp :type Primitive%20Component%20Object%20Reference) (OtherBodyIndex :type Integer) (bFromSweep :type Boolean) (SweepResult :type Hit%20Result%20Structure%20%28by%20ref%29))
  ;[1 1 1] Basic Collision Mechanics
  (bind _asbcharacter (Utilities|Casting|CastToBCharacter OtherActor))
  (Utilities|FlowControl|DoOnce false
    (:Completed
      (bind (_outhit _returnvalue) (Collision|LineTraceForObjects 0 (Transformation|GetWorldLocation (Variables|Default|GetHitDetect)) (Transformation|GetWorldLocation (Variables|Default|GetHitDetect2)) (Utilities|Array|MakeArray "ObjectTypeQuery3") false 0 "ForDuration"))
      (if _returnvalue
        (Physics|SetSimulatePhysics (.HitComponent (Collision|BreakHitResult _outhit)) true)
        (bind _output_get (Variables|Default|SetHitBone (.HitBoneName (Collision|BreakHitResult _outhit))))
        (Class|PhysicsConstraintComponent|SetConstrainedComponents (Variables|Default|GetPhysicsConstraint) (Variables|Default|GetHitDetect) "None" (.HitComponent (Collision|BreakHitResult _outhit)) _output_get)
        (Collision|SetCollisionResponsetoAllChannels (Variables|Default|GetHitDetect) "ECR_Ignore")
        (Variables|Default|SetHitMesh (Variables|/Script/Engine.Character|GetMesh _asbcharacter))))))

(fn ConstructionScript)