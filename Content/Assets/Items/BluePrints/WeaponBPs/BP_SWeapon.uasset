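; BP_SWeapon is a weapon item that a BCharacter can pick up and carry in a holster.
; Its OverlapDetect component enables input on the weapon for player 0 while a character overlaps, and disables it on exit.
; Pressing F when the character holds no item turns off collision and physics, attaches the weapon to the WeaponHolster mesh socket, registers it on the character and disables its input.
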(event OnComponentBeginOverlap(OverlapDetect)
  (params (OtherActor :type Actor%20Object%20Reference) (OtherComp :type Primitive%20Component%20Object%20Reference) (OtherBodyIndex :type Integer) (bFromSweep :type Boolean) (SweepResult :type Hit%20Result%20Structure%20%28by%20ref%29))
  ;[1 1 1] Enable/Disable Input
  (Utilities|Casting|CastToBCharacterClass (Utilities|GetClass OtherActor))
  (Development|PrintString 0 "ENTERING!!!!!")
  (Input|EnableInput (Game|GetPlayerController 0)))

(event OnComponentEndOverlap(OverlapDetect)
  (params (OtherActor :type Actor%20Object%20Reference) (OtherComp :type Primitive%20Component%20Object%20Reference) (OtherBodyIndex :type Integer))
  ;[1 1 1] Enable/Disable Input
  (Utilities|Casting|CastToBCharacterClass (Utilities|GetClass OtherActor))
  (Development|PrintString 0 "Exiting!!!!!!!")
  (Input|DisableInput (Game|GetPlayerController 0)))

(event Input|KeyboardEvents|F
  (params (Key :type Key%20Structure :default "AnyKey"))
  ;[1 1 1] Pickup Item
  (:Pressed
    (bind _asbcharacter (Utilities|Casting|CastToBCharacter (stale OnComponentBeginOverlap(OverlapDetect) OtherActor))
      (:then
        (if (Variables|/Script/BrensFullGame.BCharacter|GetIsItemHeld _asbcharacter)
          (Development|PrintString 0 "E5")
          (else
            (CallFunction|SetCollision false)
            (Class|Actor|AttachRootComponentto (Variables|/Script/Engine.Character|GetMesh _asbcharacter) "WeaponHolster" "SnapToTarget" true)
            (Class|BCharacter|SetValues _asbcharacter self (Variables|Default|GetItemType) true)
            (Input|DisableInput (Game|GetPlayerController 0)))))
      (:CastFailed
        (Development|PrintString 0 "E4")))))

(fn ConstructionScript)

(fn SetCollision
  (params (On? :type Boolean))
  (if On?
    (Variables|Default|SetEnableCollisionE "QueryAndPhysics")
    (else
      (Variables|Default|SetEnableCollisionE "NoCollision")))
  (Collision|SetCollisionEnabled (Variables|Default|GetOverlap%20Detect) (Variables|Default|GetEnableCollisionE))
  (Physics|SetSimulatePhysics (Variables|Default|GetSItemMesh) On?))