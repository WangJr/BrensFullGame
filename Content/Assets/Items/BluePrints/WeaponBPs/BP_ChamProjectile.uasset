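; Thrown weapon projectile (a knife) that impales characters and can pin them to world geometry.
; On Tick, a Hilt-side pawn trace ragdolls the struck character, constrains the hit bone to the projectile and kills AI.
; Tip-side traces, bridged from the previous tip position, detect static world hits.
; On impact it spawns the saved weapon class in its place, transfers any impaled body's constraint and destroys itself.
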(event EventTick
  (params (DeltaSeconds :type Float%20%28single-precision%29))
  (bind _projectilemesh (Variables|Default|GetProjectileMesh))
  (bind _returnvalue (Transformation|GetSocketLocation _projectilemesh "Tip"))
  (bind _returnvalue_2 (Transformation|GetSocketLocation _projectilemesh "Hilt"))
  ;[1 1 1] Only Run if Trace is required
  (if (Variables|Default|GetbTrace?)
    ;[1 1 1] Look To See if a Character has been Impaled. True = Only Look for WS, False = Look for both
    (if (Variables|Default|GetbImpaled?)
      ;[1 1 1] World Trace from 75% to Tip
      (bind (_s _f) (CallFunction|CalculateTraceZone true _returnvalue _returnvalue_2 :!label _label))
      (bind _hit_ (CallFunction|RunTracesforWorld _s _f))
      (if _hit_
        (CallFunction|SpawnBP :!label _label_2))
      (else
        ;[1 1 1] Pawn Trace from Hilt to 25%
        (bind (_s_2 _f_2) (CallFunction|CalculateTraceZone false _returnvalue _returnvalue_2))
        (bind (_outhit _returnvalue_3) (Collision|LineTraceForObjects 0 _s_2 _f_2 (Utilities|Array|MakeArray "ObjectTypeQuery3") false 0 "ForDuration"))
        (if _returnvalue_3
          ;[1 1 1] World Trace from 75%-Tip
          (bind (_s_3 _f_3) (CallFunction|CalculateTraceZone true _returnvalue _returnvalue_2))
          (bind _hit__2 (CallFunction|RunTracesforWorld _s_3 _f_3))
          ;[1 1 1] If Character is detected in Trace, Attach to Hilt Socket, Set Implaed to TRUE
          (bind _asbcharacter (Utilities|Casting|CastToBCharacter (.HitActor (Collision|BreakHitResult _outhit))))
          (Physics|SetSimulatePhysics (Variables|/Script/Engine.Character|GetMesh _asbcharacter) true)
          (bind _output_get (Variables|Default|SetHitBone (.HitBoneName (Collision|BreakHitResult _outhit))))
          (Class|PhysicsConstraintComponent|SetConstrainedComponents (Variables|Default|GetPhysicsConstraint) (Variables|Default|GetProjectileMesh) "Hilt" (.HitComponent (Collision|BreakHitResult _outhit)) _output_get)
          (Variables|Default|SetHitMesh (Variables|/Script/Engine.Character|GetMesh _asbcharacter))
          (Variables|Default|SetbImpaled? true)
          (bind _asaitemplate (Utilities|Casting|CastToAITemplate _asbcharacter))
          (Default|DIDeath _asaitemplate)
          (if _hit__2
            (goto _label_2))
          (else
            (goto _label)))))))

(fn ConstructionScript
  (Variables|Default|SetOld%20Tip (Transformation|GetWorldLocation (Variables|Default|GetHitDetect))))

(fn CalculateTraceZone
  (params (PlayerHit? :type Boolean) (TheTip :type Vector) (TheHilt :type Vector))
  (bind _returnvalue (- TheTip TheHilt))
  (if PlayerHit?
    (LocalVariables|SetStart (+ (* _returnvalue 0.75) TheHilt))
    (LocalVariables|SetFinish TheTip)
    (else
      (LocalVariables|SetStart TheHilt)
      (LocalVariables|SetFinish (+ (* _returnvalue 0.25) TheHilt))))
  (return (LocalVariables|GetStart) (LocalVariables|GetFinish)))

(fn RunTracesforWorld
  (params (S :type Vector) (F :type Vector))
  (bind _array (Utilities|Array|MakeArray "ObjectTypeQuery1"))
  (bind (_outhit _returnvalue) (Collision|LineTraceForObjects 0 (Variables|Default|GetOld%20Tip) S _array false 0 "ForDuration"))
  (if _returnvalue
    (Variables|Default|SetStaticHit (.Location (Collision|BreakHitResult _outhit)))
    (LocalVariables|SetbHit? true)
    (else
      (bind (_outhit_2 _returnvalue_2) (Collision|LineTraceForObjects 0 S F _array false 0 "ForDuration"))
      (if _returnvalue_2
        (Variables|Default|SetStaticHit (.Location (Collision|BreakHitResult _outhit_2)))
        (LocalVariables|SetbHit? true)
        (else
          (Variables|Default|SetOld%20Tip F)
          (LocalVariables|SetbHit? false)))))
  (return (LocalVariables|GetbHit?)))

(fn SpawnBP
  (bind _projectilemovement (Variables|Default|GetProjectileMovement))
  ;[1 1 1] Immediately Stop All Motion on a World Static Hit
  (Components|Movement|StopMovementImmediately _projectilemovement)
  (Variables|/Script/Engine.ProjectileMovementComponent|SetbRotationFollowsVelocity _projectilemovement false)
  ;[1 1 1] Spawn BP of Saved SWeapon Class
  (bind _returnvalue (Game|SpawnActorfromClass (Variables|Default|GetBPClass) (Transformation|GetWorldTransform (Variables|Default|GetProjectileMesh)) "AlwaysSpawn" 0 0))
  ;[1 1 1] Physics is Set to Simulate by default. Since knife is stuck, we don't need physics
  (Physics|SetSimulatePhysics (Variables|/Script/BrensFullGame.SItem|GetSItemMesh _returnvalue) false)
  ;[1 1 1] Break Constraint on Projectile and Attach to Spawned Knife
  (Class|PhysicsConstraintComponent|BreakConstraint (Variables|Default|GetPhysicsConstraint))
  (Class|PhysicsConstraintComponent|SetConstrainedComponents (Variables|/Game/Assets/Items/BluePrints/WeaponBPs/BP_SWeapon.BP_SWeapon_C|GetImpalor _returnvalue) (Variables|/Script/BrensFullGame.SItem|GetSItemMesh _returnvalue) "Hilt" (Variables|Default|GetHitMesh) (Variables|Default|GetHitBone))
  (Class|PhysicsConstraintComponent|SetDisableCollision (Variables|/Game/Assets/Items/BluePrints/WeaponBPs/BP_SWeapon.BP_SWeapon_C|GetImpalor _returnvalue) true)
  ;[1 1 1] We Want no more calls to Tick
  (Variables|Default|SetbTrace? false)
  ;[1 1 1] If Actor is Impaled in AI/Player, do not allow Handle Collision to Turn on, then DESTROY PROJECTILE
  (if (Variables|Default|GetbImpaled?)
    (Variables|/Game/Assets/Items/BluePrints/WeaponBPs/BP_SWeapon.BP_SWeapon_C|SetbImpaled? _returnvalue true)
    (else
      (Variables|/Game/Assets/Items/BluePrints/WeaponBPs/BP_SWeapon.BP_SWeapon_C|SetbStuckWS? _returnvalue true)
      (Default|ToggleCollision _returnvalue)
      (Variables|Default|SetbImpaled? false)))
  (Actor|DestroyActor))